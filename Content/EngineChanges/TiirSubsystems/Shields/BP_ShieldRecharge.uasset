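; BP_ShieldRecharge is the visual for a shield's recharge state, fading a shield mesh in while recharging and out otherwise.
; On init it adds the supplied mesh without shadows or collision and creates a dynamic material instance with the fade and impact wave parameters zeroed.
; An update event sets the Recharging flag, and Tick lerps the material's Fade toward it at a rate scaled by ShieldSpeed.
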(event EventShieldInitRecharge
  (params (Mesh :type Static%20Mesh%20Object%20Reference))
  (bind _returnvalue (AddComponent|AddStaticMeshComponent false))
  (Rendering|SetCastShadow _returnvalue false)
  (Collision|SetCollisionEnabled _returnvalue "NoCollision")
  (Components|StaticMesh|SetStaticMesh _returnvalue Mesh)
  (bind _returnvalue_2 (Rendering|Material|CreateDynamicMaterialInstance _returnvalue 0 (Rendering|Material|GetMaterial Mesh 0) "None" :!class /Script/Engine.PrimitiveComponent))
  (bind _output_get (Variables|Default|SetDynamicMaterialInstance _returnvalue_2))
  (Rendering|Material|SetScalarParameterValue _output_get "Fade" 0.0 :!class /Script/Engine.MaterialInstanceDynamic)
  (Rendering|Material|SetScalarParameterValue _output_get "UseImpactWave" 0.0 :!class /Script/Engine.MaterialInstanceDynamic))

(event EventShieldUpdateRecharge
  (params (Recharging :type Boolean))
  (Variables|Default|SetRecharging Recharging))

(event EventTick
  (params (DeltaSeconds :type Float%20%28single-precision%29))
  (if (!= (Variables|Default|GetFadeValue) (Math|Conversions|ToFloat(Boolean) (Variables|Default|GetRecharging)))
    (bind _output_get (Variables|Default|SetFadeValue (Math|Float|Lerp (Variables|Default|GetFadeValue) (Math|Conversions|ToFloat(Boolean) (Variables|Default|GetRecharging)) (* DeltaSeconds (Variables|Default|GetShieldSpeed)))))
    (Rendering|Material|SetScalarParameterValue (Variables|Default|GetDynamicMaterialInstance) "Fade" _output_get :!class /Script/Engine.MaterialInstanceDynamic)))

(fn ConstructionScript)