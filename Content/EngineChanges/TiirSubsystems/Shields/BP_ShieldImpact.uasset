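; BP_ShieldImpact is a short-lived effect actor that shows an expanding impact wave where a shield is hit.
; ShieldHit adds a shadowless, collision-free copy of the supplied mesh and gives it a dynamic material instance with the hit location in actor-local space.
; A timeline grows the impact radius, scaled by the hit size, while driving Fade inversely, then the actor destroys itself when it finishes.
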(event EventShieldHit
  (params (Location :type Vector :default "0, 0, 0") (Size :type Float%20%28single-precision%29) (Mesh :type Static%20Mesh%20Object%20Reference))
  (bind _returnvalue (AddComponent|AddStaticMeshComponent false))
  (Rendering|SetCastShadow _returnvalue false)
  (Collision|SetCollisionEnabled _returnvalue "NoCollision")
  (Components|StaticMesh|SetStaticMesh _returnvalue Mesh)
  (bind _returnvalue_2 (Rendering|Material|CreateDynamicMaterialInstance _returnvalue 0 (Rendering|Material|GetMaterial Mesh 0) "None" :!class /Script/Engine.PrimitiveComponent))
  (Rendering|Material|SetVectorParameterValue _returnvalue_2 "POS" (Math|Conversions|ToLinearColor(Vector) (Math|Transform|InverseTransformLocation (Transformation|GetActorTransform) Location)) :!class /Script/Engine.MaterialInstanceDynamic)
  (Rendering|Material|SetScalarParameterValue _returnvalue_2 "UseImpactWave" 1.0 :!class /Script/Engine.MaterialInstanceDynamic)
  (bind _impact (Timeline|Timeline_0 PlayFromStart)
    (:Update
      (Rendering|Material|SetScalarParameterValue _returnvalue_2 "Fade" (- 1.0 _impact) :!class /Script/Engine.MaterialInstanceDynamic)
      (Rendering|Material|SetScalarParameterValue _returnvalue_2 "ImpactRadius" (* _impact Size) :!class /Script/Engine.MaterialInstanceDynamic))
    (:Finished
      (Actor|DestroyActor))))

(fn ConstructionScript)