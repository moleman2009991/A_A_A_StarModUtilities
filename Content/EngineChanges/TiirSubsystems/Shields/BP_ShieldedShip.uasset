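; Ship Blueprint that adds shield behavior: hit effects, a recharge glow and helpers for shield damage.
; Hits spawn a damage-sized child-actor effect while shields hold, and a dynamic material fades the shield mesh in during regeneration.
; Helper functions match projectiles to owner weapon data for penetration, split damage between shield and hull, and ease regeneration.
; Hull splat damage only applies once shields are nearly depleted.
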(event EventBeginPlay
  (bind _shieldmesh (Variables|ShieldConfig|GetShieldMesh))
  (|CallParentFunction)
  (if (Variables|ShieldConfig|GetShowShieldsWhenRecharging)
    (bind _returnvalue (AddComponent|AddStaticMeshComponent false))
    (Rendering|SetCastShadow _returnvalue false)
    (Collision|SetCollisionEnabled _returnvalue "NoCollision")
    (Components|StaticMesh|SetStaticMesh _returnvalue _shieldmesh)
    (bind _returnvalue_2 (Rendering|Material|CreateDynamicMaterialInstance _returnvalue 0 (Rendering|Material|GetMaterial _shieldmesh 0) "None" :!class /Script/Engine.PrimitiveComponent))
    (bind _output_get (Variables|Default|SetShieldMaterialInstance _returnvalue_2))
    (Rendering|Material|SetScalarParameterValue _output_get "Fade" 0.0 :!class /Script/Engine.MaterialInstanceDynamic)
    (Rendering|Material|SetScalarParameterValue _output_get "UseImpactWave" 0.0 :!class /Script/Engine.MaterialInstanceDynamic)))

(event EventUpdateShieldHealthValue
  (params (New%20Health%20Value :type Float%20%28single-precision%29))
  (Default|SetNewShieldHealth (Variables|Default|GetShieldHealthComponent) New%20Health%20Value))

(event EventTick
  (params (DeltaSeconds :type Float%20%28single-precision%29))
  (bind _self self)
  (|CallParentFunction DeltaSeconds)
  (if (Variables|ShieldConfig|GetShowShieldsWhenRecharging)
    (Variables|Default|SetRecharging (Math|Boolean|ANDBoolean (Variables|/A_A_A_StarModUtilities/EngineChanges/TiirSubsystems/Shields/ShieldHealthComponent.ShieldHealthComponent_C|GetRegenCurrently (Variables|Default|GetShieldHealthComponent)) (Class|SimEntity|CanbeFocused) (Class|RavenSelectionUtils|CanCurrentlybeHovered _self) (Class|RavenSelectionUtils|CanCurrentlybeSelected _self) (not (Variables|Default|GetIsDocked _self))))
    (if (!= (Variables|Default|GetFadeValue) (Math|Conversions|ToFloat(Boolean) (Variables|Default|GetRecharging)))
      (bind _output_get (Variables|Default|SetFadeValue (Math|Float|Lerp (Variables|Default|GetFadeValue) (Math|Conversions|ToFloat(Boolean) (Variables|Default|GetRecharging)) (* DeltaSeconds (Variables|Default|GetShieldSpeed)))))
      (Rendering|Material|SetScalarParameterValue (Variables|Default|GetShieldMaterialInstance) "Fade" _output_get :!class /Script/Engine.MaterialInstanceDynamic))))

(event EventSimDamage
  (params (Player :type Sim%20Player%20Object%20Reference) (HitEntity :type Sim%20Entity%20Object%20Reference) (AttackingEntity :type Sim%20Entity%20Object%20Reference) (DamagePosition :type Vector :default "0, 0, 0") (DamageNormal :type Vector :default "0, 0, 0") (HitDirectionMultiplierType :type EWeaponHitDirectionMultiplierType%20Enum :default "None") (DamageType :type EWeaponFireType%20Enum :default "Bullet") (DamageAmount :type Integer))
  (if (== self HitEntity)
    (Utilities|FlowControl|Sequence
      (:then_0
        ;[1 0.4357 0] Create shield FX
        (if (> (Math|Float|Truncate (Variables|/A_A_A_StarModUtilities/EngineChanges/TiirSubsystems/Shields/ShieldHealthComponent.ShieldHealthComponent_C|GetCurrent%20Health (Variables|Default|GetShieldHealthComponent))) 0)
          (bind _returnvalue (AddComponent|AddChildActorComponent false))
          (Class|BPIShieldImpact|ShieldHit(Message) (Variables|/Script/Engine.ChildActorComponent|GetChildActor _returnvalue) DamagePosition (CallFunction|GetDamageShieldFxSize DamageAmount) (Variables|ShieldConfig|GetShieldMesh))))
      (:then_2
        (|CallParentFunction Player HitEntity AttackingEntity DamagePosition DamageNormal HitDirectionMultiplierType DamageType DamageAmount :!label _label)))
    (else
      (goto _label))))

(fn ConstructionScript
  (|CallParentFunction))

(fn GetProjectileShieldPenetrationandDamageMultiplier
  (params (Projectile :type Sim%20Entity%20Object%20Reference))
  (bind _asbp_projectile (Utilities|Casting|CastToBP_Projectile Projectile)
    (:then
      (bind _asbp_ship (Utilities|Casting|CastToBP_Ship (Variables|/Script/RavenSimulation.WeaponFireActor|GetOwnerShipActor _asbp_projectile))
        (:then
          (bind _array_element (Utilities|Array|ForEachLoopwithBreak (Variables|/Script/RavenSimulation.ShipStaticData|GetWeapons (Variables|/Script/RavenSimulation.SimShip|GetDataAsset _asbp_ship)))
            (:LoopBody
              (bind _array_element_2 (Utilities|Array|ForEachLoopwithBreak (.weapons _array_element))
                (:LoopBody
                  (if (== (Variables|/Script/RavenSimulation.WeaponFireActor|GetDataAsset _asbp_projectile) (Variables|/Script/RavenSimulation.WeaponStaticData|GetWeaponFireData _array_element_2))
                    (return (Variables|/Script/RavenSimulation.WeaponStaticData|GetShieldPenetrationMultipler _array_element_2) (Variables|/Script/RavenSimulation.WeaponStaticData|GeteWeaponShieldPenetration _array_element_2))))
                (:Completed
                  (if (== (Variables|/Script/RavenSimulation.WeaponFireActor|GetDataAsset _asbp_projectile) (Variables|/Script/RavenSimulation.WeaponStaticData|GetWeaponFireData (.weapon _array_element)))
                    (return (Variables|/Script/RavenSimulation.WeaponStaticData|GetShieldPenetrationMultipler (.weapon _array_element)) (Variables|/Script/RavenSimulation.WeaponStaticData|GeteWeaponShieldPenetration (.weapon _array_element)))))))
            (:Completed
              (return 0.0 "None"))))
        (:CastFailed
          (return 0.0 "None"))))
    (:CastFailed
      (return 0.0 "None"))))

(fn ComputeShieldPenetration
  (params (Shield%20Penetration%20Type :type EWeaponShieldPenetration%20Enum :default "None"))
  (return (Utilities|Select :Index Shield%20Penetration%20Type :None 0.0 :Normal 0.5 :Enhanced 0.75 :Bypass 1.0)))

(fn GetProjectileShieldPenetration
  (params (Projectile :type Sim%20Entity%20Object%20Reference))
  (bind _asweapon_fire_actor (Utilities|Casting|CastToWeaponFireActor Projectile)
    (:then
      ;[1 1 1] Set Local Projectile Data Asset Variable
      (LocalVariables|SetProjectile%20DA (Variables|/Script/RavenSimulation.WeaponFireActor|GetDataAsset _asweapon_fire_actor))
      (bind _asbp_ship (Utilities|Casting|CastToBP_Ship (Variables|/Script/RavenSimulation.WeaponFireActor|GetOwnerShipActor _asweapon_fire_actor))
        (:then
          ;[0 0 1] Set Local Weapon Attachments to Array So we don't have to re-cast when checking the Array
          (bind _output_get (LocalVariables|SetFound%20Weapon%20Attachments (Variables|/Script/RavenSimulation.ShipStaticData|GetWeapons (Variables|/Script/RavenSimulation.SimShip|GetDataAsset _asbp_ship))))
          (bind _index (Utilities|FlowControl|ForLoopwithBreak 0 (- (Utilities|Array|Length _output_get) 1))
            (:LoopBody
              (if (== (LocalVariables|GetProjectile%20DA) (Variables|/Script/RavenSimulation.WeaponStaticData|GetWeaponFireData (.weapon (Utilities|Array|Get(acopy) _output_get _index))))
                (LocalVariables|SetFound%20Shield%20PT (Variables|/Script/RavenSimulation.WeaponStaticData|GeteWeaponShieldPenetration (.weapon (Utilities|Array|Get(acopy) _output_get _index))))
                (LocalVariables|SetFound%20Sheild%20PM (Variables|/Script/RavenSimulation.WeaponStaticData|GetShieldPenetrationMultipler (.weapon (Utilities|Array|Get(acopy) _output_get _index))))
                (return (LocalVariables|GetFound%20Shield%20PT) (LocalVariables|GetFound%20Sheild%20PM))
                (else
                  (bind _index_2 (Utilities|FlowControl|ForLoopwithBreak 0 (- (Utilities|Array|Length (.weapons (Utilities|Array|Get(acopy) _output_get _index))) 1))
                    (:LoopBody
                      (if (== (LocalVariables|GetProjectile%20DA) (Variables|/Script/RavenSimulation.WeaponStaticData|GetWeaponFireData (Utilities|Array|Get(acopy) (.weapons (Utilities|Array|Get(acopy) _output_get _index)) _index_2)))
                        (LocalVariables|SetFound%20Shield%20PT (Variables|/Script/RavenSimulation.WeaponStaticData|GeteWeaponShieldPenetration (Utilities|Array|Get(acopy) (.weapons (Utilities|Array|Get(acopy) _output_get _index)) _index_2)))
                        (LocalVariables|SetFound%20Sheild%20PM (Variables|/Script/RavenSimulation.WeaponStaticData|GetShieldPenetrationMultipler (Utilities|Array|Get(acopy) (.weapons (Utilities|Array|Get(acopy) _output_get _index)) _index_2)))
                        (return (LocalVariables|GetFound%20Shield%20PT) (LocalVariables|GetFound%20Sheild%20PM))))))))
            (:Completed
              (return "None" 1.0))))
        (:CastFailed
          (return "None" 1.0))))
    (:CastFailed
      (return "None" 1.0))))

(fn SetShipHealth)

(fn ComputeDamages
  (params (Shield%20penetration%20type :type EWeaponShieldPenetration%20Enum :default "None") (Shield%20damage%20multiplier :type Float%20%28single-precision%29) (Damage :type Integer))
  (LocalVariables|SetShield%20Penetration%20Multiplier (Utilities|Select :Index Shield%20penetration%20type :None 0.0 :Normal 0.5 :Enhanced 0.75 :Bypass 1.0))
  (LocalVariables|SetIncoming%20damage (Math|Conversions|ToFloat(Integer) Damage))
  (return (Math|Float|Max(Float) (- (Variables|/A_A_A_StarModUtilities/EngineChanges/TiirSubsystems/Shields/ShieldHealthComponent.ShieldHealthComponent_C|GetCurrent%20Health (Variables|Default|GetShieldHealthComponent)) (* (* Shield%20damage%20multiplier (- 1.0 (LocalVariables|GetShield%20Penetration%20Multiplier))) (LocalVariables|GetIncoming%20damage))) 0.0) (+ (Math|Float|Max(Float) (- (* (- 1.0 (LocalVariables|GetShield%20Penetration%20Multiplier)) (LocalVariables|GetIncoming%20damage)) (Variables|/A_A_A_StarModUtilities/EngineChanges/TiirSubsystems/Shields/ShieldHealthComponent.ShieldHealthComponent_C|GetCurrent%20Health (Variables|Default|GetShieldHealthComponent))) 0.0) (* (LocalVariables|GetShield%20Penetration%20Multiplier) (LocalVariables|GetIncoming%20damage)))))

(fn GetDamageShieldFxSize
  (params (Damages :type Integer))
  (return (* (Math|Conversions|ToFloat(Integer) (+ Damages 50)) (Variables|ShieldConfig|GetShieldFX_SizeMultiplier))))

(fn ShieldRegenerationEase
  (params (NormalizedHealth :type Float%20%28single-precision%29) (TimeSinceRegenStart :type Float%20%28single-precision%29))
  (return (- (Math|Float|Clamp(Float) (* (Math|Float|Clamp(Float) (- 1.0 (* (Math|Float|Power (/ (- (Math|Float|Clamp(Float) NormalizedHealth 0.85) 0.85) 0.15) 2.0) 0.8)) 0.2) (Math|Float|Clamp(Float) (- 1.0 (Math|Float|Power 0.8 (Class|KismetMathLibrary|Exp (* (Math|Float|Clamp(Float) TimeSinceRegenStart 0.0 2.0) -2.191)))) 0.2)) 0.2) 0.2)))

(fn OnRepSimDamageReceived)

(fn ApplySplatDamage
  (params (HitLocation :type Vector :default "0, 0, 0") (BrushColor :type Linear%20Color%20Structure) (BrushSize :type Float%20%28single-precision%29) (BrushTextureRotationDegrees :type Float%20%28single-precision%29) (BrushTexture :type Texture%202D%20Object%20Reference) (InLocalSpace :type Boolean))
  (if (<= (Default|GetNormalizedHealth (Variables|Default|GetShieldHealthComponent)) 0.05)
    (|CallParentFunction HitLocation BrushColor BrushSize BrushTextureRotationDegrees BrushTexture InLocalSpace)))