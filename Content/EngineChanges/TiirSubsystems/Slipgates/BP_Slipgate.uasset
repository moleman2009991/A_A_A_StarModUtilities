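; BP_Slipgate is a slipgate actor with a portal mesh and entrance and exit sphere volumes taken from child actors.
; Construction and TiirStartup both build a dynamic portal material with local/destination textures and colors, and scale the entrance; startup also caches both volumes.
; Logic to teleport player ships entering the gate and turn the arrow toward the nearer camera is disconnected, and ticking does nothing.
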(event EventTiirStartup
  (bind _entrancescale (Variables|Default|GetEntranceScale))
  (bind _mat_1 (Variables|Default|GetMat_1))
  (Utilities|FlowControl|Sequence
    (:then_0
      (bind _assim_sphere_volume (Utilities|Casting|CastToSimSphereVolume (Variables|/Script/Engine.ChildActorComponent|GetChildActor (Variables|Default|GetEntrance))))
      (Variables|Default|SetEntrance%20Point _assim_sphere_volume)
      (bind _assim_sphere_volume_2 (Utilities|Casting|CastToSimSphereVolume (Variables|/Script/Engine.ChildActorComponent|GetChildActor (Variables|Default|GetExit))))
      (Variables|Default|SetExit%20Point _assim_sphere_volume_2)
      (Rendering|Material|SetMaterial (Variables|Default|GetStaticMesh) 0 _mat_1)
      (bind _returnvalue (Rendering|Material|CreateDynamicMaterialInstance (Variables|Default|GetStaticMesh) 0 _mat_1 "None" :!class /Script/Engine.PrimitiveComponent))
      (Variables|Default|SetDMI_1 _returnvalue)
      (Rendering|Material|SetTextureParameterValue (Variables|Default|GetDMI_1) "TC_LocalSpace" (Variables|Default|GetTC_LocalSpace))
      (Rendering|Material|SetTextureParameterValue (Variables|Default|GetDMI_1) "TC_Destination" (Variables|Default|GetTC_Destination))
      (Rendering|Material|SetVectorParameterValue (Variables|Default|GetDMI_1) "Color_Inner" (Variables|Default|GetColor_Inner) :!class /Script/Engine.MaterialInstanceDynamic)
      (Rendering|Material|SetVectorParameterValue (Variables|Default|GetDMI_1) "Color_Outer" (Variables|Default|GetColor_Outer) :!class /Script/Engine.MaterialInstanceDynamic)
      (Rendering|Material|SetVectorParameterValue (Variables|Default|GetDMI_1) "Color_Waves_1" (Variables|Default|GetColor_Waves_1) :!class /Script/Engine.MaterialInstanceDynamic)
      (Rendering|Material|SetVectorParameterValue (Variables|Default|GetDMI_1) "Color_Waves_2" (Variables|Default|GetColor_Waves_2) :!class /Script/Engine.MaterialInstanceDynamic)
      ;[1 1 1] Entrance location
      (Transformation|SetRelativeScale3D (Variables|Default|GetEntrance) (Math|Vector|MakeVector _entrancescale _entrancescale _entrancescale)))))

(event EventTiirTick)

(event EventTick
  (params (DeltaSeconds :type Float%20%28single-precision%29))
  ;[1 1 1] Set rotation: look at player camera
)

(fn ConstructionScript
  (bind _entrancescale (Variables|Default|GetEntranceScale))
  (bind _mat_1 (Variables|Default|GetMat_1))
  (Rendering|Material|SetMaterial (Variables|Default|GetStaticMesh) 0 _mat_1)
  (bind _returnvalue (Rendering|Material|CreateDynamicMaterialInstance (Variables|Default|GetStaticMesh) 0 _mat_1 "None" :!class /Script/Engine.PrimitiveComponent))
  (Variables|Default|SetDMI_1 _returnvalue)
  (Rendering|Material|SetTextureParameterValue (Variables|Default|GetDMI_1) "TC_LocalSpace" (Variables|Default|GetTC_LocalSpace))
  (Rendering|Material|SetTextureParameterValue (Variables|Default|GetDMI_1) "TC_Destination" (Variables|Default|GetTC_Destination))
  (Rendering|Material|SetVectorParameterValue (Variables|Default|GetDMI_1) "Color_Inner" (Variables|Default|GetColor_Inner) :!class /Script/Engine.MaterialInstanceDynamic)
  (Rendering|Material|SetVectorParameterValue (Variables|Default|GetDMI_1) "Color_Outer" (Variables|Default|GetColor_Outer) :!class /Script/Engine.MaterialInstanceDynamic)
  (Rendering|Material|SetVectorParameterValue (Variables|Default|GetDMI_1) "Color_Waves_1" (Variables|Default|GetColor_Waves_1) :!class /Script/Engine.MaterialInstanceDynamic)
  (Rendering|Material|SetVectorParameterValue (Variables|Default|GetDMI_1) "Color_Waves_2" (Variables|Default|GetColor_Waves_2) :!class /Script/Engine.MaterialInstanceDynamic)
  (Transformation|SetRelativeScale3D (Variables|Default|GetEntrance) (Math|Vector|MakeVector _entrancescale _entrancescale _entrancescale)))

(fn GetTiirTickEnabled
  (return false))

(fn GetTiirTickInterval
  (return 0.0))