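; Editor-side cinematic path visualizer that previews a unit mesh or camera at a chosen point on a spline, built entirely in the construction script.
; It creates or removes skeletal mesh, static mesh and spring-arm cine camera components under MeshRoot, gated by DoOnce toggles.
; MeshRoot snaps to the selected spline point.
; The camera applies zoom, offset and arm settings, then aims at another visualizer, which records it for focus tracking.
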(event EventBeginPlay)

(event Collision|EventActorBeginOverlap
  (params (OtherActor :type Actor%20Object%20Reference)))

(event EventTick
  (params (DeltaSeconds :type Float%20%28single-precision%29)))

(fn ConstructionScript
  (bind (_zoom _x_offset _y_offset _roll _pitch _yaw _aspect_ratio _field_of_view) (Utilities|Utility-GetCameraSettings))
  (bind _custompath (Variables|Default|GetCustomPath))
  (bind _ship_position_on_spline (Variables|Default|GetShip%20Position%20On%20Spline))
  (bind _camera_focus_actor (Variables|Camera|GetCamera%20Focus%20Actor))
  (bind _meshroot (Variables|Default|GetMeshRoot))
  (bind _returnvalue (Transformation|GetWorldRotation _meshroot))
  (bind _returnvalue_2 (- _ship_position_on_spline 1))
  (bind _returnvalue_3 (Spline|GetNumberOfSplinePoints _custompath))
  (bind _meshroot_2 (Variables|BP_Cina_UnitPathVisualizer_C|GetMeshRoot _camera_focus_actor))
  (bind _returnvalue_4 (Transformation|GetWorldLocation _meshroot_2))
  (Utilities|FlowControl|Sequence
    (:then_0
      ;[1 1 1] Initial Setup of Meshes
      (Utilities|FlowControl|Sequence
        (:then_0
          ;[1 1 1] Setup & Display Initial Skeletal Mesh if Valid
          (Utilities|IsValid (Variables|Components|GetSkeletal%20Mesh%20to%20Use)
            (:Is%20Valid
              (Utilities|FlowControl|Sequence
                (:then_0
                  (goto _label_2 Reset))
                (:then_1
                  (Utilities|FlowControl|DoOnce false :!label _label
                    (:Completed
                      (bind _returnvalue_5 (AddComponent|AddSkeletalMeshComponent true))
                      (bind _output_get (LocalVariables|SetCreated%20SKMesh _returnvalue_5))
                      (Transformation|AttachComponentToComponent _output_get (Variables|Default|GetMeshRoot) "None" "KeepRelative" "KeepRelative" "KeepRelative" true)
                      (Class|SkinnedMeshComponent|SetSkeletalMesh _output_get (Variables|Components|GetSkeletal%20Mesh%20to%20Use) true)
                      (Transformation|SetWorldRotation _output_get _returnvalue false false))))))
            (:Is%20Not%20Valid
              (Utilities|FlowControl|DoOnce false :!label _label_2
                (:Completed
                  (Utilities|IsValid (LocalVariables|GetCreated%20SKMesh)
                    (:Is%20Valid
                      (Components|DestroyComponent (LocalVariables|GetCreated%20SKMesh))
                      (goto _label Reset))))))))
        (:then_1
          ;[1 1 1] Setup & Display Initial Static Mesh if Valid
          (Utilities|IsValid (Variables|Components|GetStatic%20Mesh%20to%20Use)
            (:Is%20Valid
              (Utilities|FlowControl|Sequence
                (:then_0
                  (goto _label_4 Reset))
                (:then_1
                  (Utilities|FlowControl|DoOnce false :!label _label_3
                    (:Completed
                      (bind _returnvalue_6 (AddComponent|AddStaticMeshComponent true))
                      (bind _output_get_2 (LocalVariables|SetCreates%20SMMesh _returnvalue_6))
                      (Transformation|AttachComponentToComponent _output_get_2 (Variables|Default|GetMeshRoot) "None" "KeepRelative" "KeepRelative" "KeepRelative" true)
                      (Components|StaticMesh|SetStaticMesh _output_get_2 (Variables|Components|GetStatic%20Mesh%20to%20Use))
                      (Transformation|SetWorldRotation _output_get_2 _returnvalue false false))))))
            (:Is%20Not%20Valid
              (Utilities|FlowControl|DoOnce false :!label _label_4
                (:Completed
                  (Utilities|IsValid (LocalVariables|GetCreates%20SMMesh)
                    (:Is%20Valid
                      (Components|DestroyComponent (LocalVariables|GetCreates%20SMMesh))
                      (goto _label_3 Reset))))))))))
    (:then_1
      ;[1 1 1] Setup & Display Initial Camera if Selected
      (if (Variables|Camera|GetUse%20for%20Camera?)
        (Utilities|FlowControl|Sequence
          (:then_0
            (goto _label_7 Reset))
          (:then_1
            (Utilities|FlowControl|DoOnce false :!label _label_5
              (:Completed
                (bind _returnvalue_7 (AddComponent|AddSpringArmComponent true))
                (bind _output_get_3 (Variables|Default|SetCreated%20Spring%20Arm _returnvalue_7))
                (Transformation|AttachComponentToComponent _output_get_3 (Variables|Default|GetMeshRoot) "None" "KeepRelative" "KeepRelative" "KeepRelative" true)
                (bind _returnvalue_8 (AddComponent|AddCineCameraComponent true))
                (bind _output_get_4 (Variables|Default|SetCreated%20Cina%20Camera _returnvalue_8))
                (Transformation|AttachComponentToComponent _output_get_4 (Variables|Default|GetCreated%20Spring%20Arm) "None" "KeepRelative" "KeepRelative" "KeepRelative" true)
                ;[1 1 1] Set Zoom, Offset, & Rotations
                (Utilities|Utility-SetCameraSettings (Variables|Default|GetCreated%20Cina%20Camera) (Variables|Default|GetCreated%20Spring%20Arm) (Variables|BP_Cina_UnitPathVisualizer_C|GetMeshRoot (Variables|Camera|GetCamera%20Focus%20Actor)) _zoom _x_offset _y_offset _roll _pitch _yaw _aspect_ratio _field_of_view false true :!label _label_6)))))
        (else
          (Utilities|FlowControl|DoOnce false :!label _label_7
            (:Completed
              (Utilities|IsValid (Variables|Default|GetCreated%20Cina%20Camera)
                (:Is%20Valid
                  (for _array_element (Utilities|Array|MakeArray (Variables|Default|GetCreated%20Spring%20Arm) (Variables|Default|GetCreated%20Cina%20Camera))
                    (Components|DestroyComponent _array_element))
                  (goto _label_5 Reset))))))))
    (:then_2
      ;[1 1 1] Initial Setup of Spline Point Cache w/Update Tracking
      (Utilities|FlowControl|Sequence
        (:then_0
          ;[1 1 1] Check Number of Spline Points
          (if (not (== (Variables|Default|GetCurrent%20Number%20of%20Spline%20Points) _returnvalue_3))
            ;[1 1 1] Update Number
            (Variables|Default|SetCurrent%20Number%20of%20Spline%20Points _returnvalue_3)
            ;[1 1 1] Print New Number of Points
            (Utilities|Utility-PrintNewNumberOfSplinePoints)
            ;[1 1 1] Update Ship Position
            (Utilities|Utility-UpdateShipTransformatSplinePoint :!label _label_8)
            (Utilities|IsValid (Variables|Default|GetCreated%20Cina%20Camera)
              (:Is%20Valid
                (goto _label_6)))))
        (:then_1
          ;[1 1 1] Check Position
          (if (== (- (Variables|Default|GetCurrent%20Ship%20Position) 1) _returnvalue_2)
            ;[1 1 1] Set the Ships Position First Time
            (Utilities|FlowControl|DoOnce true
              (:Completed
                (goto _label_8)))
            (else
              ;[1 1 1] Update Position
              (Variables|Default|SetCurrent%20Ship%20Position _returnvalue_2)
              (goto _label_8))))))
    (:then_3
      (Utilities|IsValid _camera_focus_actor
        (:Is%20Valid
          (if (not (Math|Vector|Equal(Vector) _returnvalue_4 (Variables|Default|GetFocus%20Actor%20Location) 0.0001))
            (Variables|BP_Cina_UnitPathVisualizer_C|SetFocus%20Actor%20Location (Variables|Camera|GetCamera%20Focusing%20On%20Actor) _returnvalue_4)
            (goto _label_6)))))))