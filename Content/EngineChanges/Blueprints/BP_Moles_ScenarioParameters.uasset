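; Scenario parameters for two-player campaign missions, running mission startup and carrying fleets between levels.
; Startup caches difficulty, plays any data-table intro animatic, then spawns persistent or default fleets using spawn types from BPI_CampaignFlow scripts and applies difficulty.
; Successful shutdown saves progress and per-player fleets, then finds the next enabled CampaignMissionData row to load or exits to menu.
; Failure shows the mission-failed panel, except on PS5, which resubmits the current level.
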(event Custom|SubmitCampaignResult_Event
  (params (PersistentFleet :type Scenario%20Fleet%20Config%20Structure) (NextLevel :type Name) (ReachedEnd :type Boolean))
  (bind _returnvalue (Utilities|String|ToString(Name) NextLevel))
  (if ReachedEnd
    (CallFunction|ExittoMainMenu)
    (else
      (for _index (range 0 1)
        (bind _returnvalue_2 (Class|RTSSaveGameSubsystem|LoadProfileSave (Subsystems|GetRTSSaveGameSubsystem)))
        (bind _returnvalue_3 (Game|ConstructObjectfromClass "/Game/Assets/Gameplay/BP_PersistentFleetSaveGame.BP_PersistentFleetSaveGame_C" _returnvalue_2))
        (bind _returnvalue_4 (Class|TiirUtilities|GetCurrentFleet (.Player (Class|TiirPlayerFunctionLibrary|GetPlayerfromIndex _index))))
        (Variables|/Game/Assets/Gameplay/BP_PersistentFleetSaveGame.BP_PersistentFleetSaveGame_C|SetFleet _returnvalue_3 _returnvalue_4)
        (bind _asraven_player_controller (Utilities|Casting|CastToRavenPlayerController (Class|GameplayStatics|GetPlayerControllerfromID _index)))
        (Utilities|IsValid (.Entities (Utilities|Struct|BreakSavedPersistentFleetEntityData (Variables|/Script/RavenSimulation.SimulationProxy|GetSavedPersistentFleetEntityData (Class|RTSPlayerController|GetSimulationProxy _asraven_player_controller))))
          (:Is%20Valid
            (Variables|/Game/Assets/Gameplay/BP_PersistentFleetSaveGame.BP_PersistentFleetSaveGame_C|SetSavedEntities _returnvalue_3 (.Entities (Utilities|Struct|BreakSavedPersistentFleetEntityData (Variables|/Script/RavenSimulation.SimulationProxy|GetSavedPersistentFleetEntityData (Class|RTSPlayerController|GetSimulationProxy _asraven_player_controller)))))
            (Class|ProfileSaveGame|SetPersistentFleetforLevel _returnvalue_2 (Utilities|String|Append "PLAYER_" (Utilities|String|ToString(Integer) _index) "_" _returnvalue) _returnvalue_3)
            (Class|RTSSaveGameSubsystem|StoreProfileSave (Subsystems|GetRTSSaveGameSubsystem)))
          (:Is%20Not%20Valid
            _))
        (Variables|Default|SetLoadedPersistentMotherships false)
        (Variables|Default|SetLoadedPersistentNonMotherships false))
      (bind _leveldata (CallFunction|GetLevelParameters _returnvalue))
      (bind _moviepaths (CallFunction|CreateMoviePaths (.loadingvideos _leveldata)))
      (Class|AsyncLoadingScreenLibrary|SetMoviePaths _moviepaths)
      (Default|CallSaveComplete (.level _leveldata)))))

(event Custom|PostAnimatic
  (params (Completed :type Boolean))
  (if (Variables|Default|GetInAnimatic)
    (Variables|Default|SetInAnimatic false)
    (for _index (range 0 1)
      (bind _asraven_player_controller (Utilities|Casting|CastToRavenPlayerController (Class|GameplayStatics|GetPlayerControllerfromID _index)))
      (Default|LetterBox _asraven_player_controller false false false 2.0)
      (if (Variables|ScenarioParameters|GetStayBlankAtStart)
        _
        (else
          (Default|HideHUD _asraven_player_controller false)))
      (Class|TiirScriptingSystem|ScheduleTiirAction (Variables|/Script/RavenSimulation.RemasteredSimulation|GetScriptingSystem (Class|SimulationDriver|GetSimulation (Variables|/Script/Raven.RTSPlayerSimComponent|GetSimDriver (Variables|/Script/Raven.RTSPlayerController|GetSimComponent _asraven_player_controller)))) 0.0)
      (Default|CallOpeningAnimaticComplete)
      (bind _objects (Class|TiirUtilities|GetTiirScriptswithInterface "/Game/Assets/Blueprints/Campaign/BPI_CampaignFlow.BPI_CampaignFlow_C"))
      (for _array_element _objects
        (bind _type (Class|BPICampaignFlow|TiirFleetSpawnType(Message) _array_element))
        (Variables|Default|SetFleetSpawnType _type))
      (CallFunction|LoadStartingFleets (Variables|Default|GetFleetSpawnType) false "ParadeHyperspace")
      (for _array_element_2 _objects
        (Class|BPICampaignFlow|TiirPostAnimatic(Message) _array_element_2 self)))))

(event Custom|StartupScenario
  (Development|PrintString "Tiir Scenario Startup" false true "(R=0.000000,G=0.660000,B=1.000000,A=1.000000)" 6e+01)
  (if (not (Variables|Default|GetInAnimatic)) ; Is an animatic currently active?
    (bind _animaticwidget (CallFunction|StartupCampaign))
    (Variables|Default|SetPassedStartupCampaign true)
    (Utilities|IsValid _animaticwidget
      (:Is%20Valid
        (Variables|Default|SetInAnimatic true)
        (EventDispatchers|BindEventtoAnimaticCompletedEvent _animaticwidget (delegate Custom|PostAnimatic)))
      (:Is%20Not%20Valid
        (Class|TiirUtilities|TiirDelay 0.2)
        (Default|CallOpeningAnimaticComplete)
        (bind _objects (Class|TiirUtilities|GetTiirScriptswithInterface "/Game/Assets/Blueprints/Campaign/BPI_CampaignFlow.BPI_CampaignFlow_C"))
        (for _array_element _objects
          (bind _type (Class|BPICampaignFlow|TiirFleetSpawnType(Message) _array_element))
          (Variables|Default|SetFleetSpawnType _type))
        (CallFunction|LoadStartingFleets (Variables|Default|GetFleetSpawnType) false "ParadeHyperspace")
        (for _array_element_2 _objects
          (Class|BPICampaignFlow|TiirPostAnimatic(Message) _array_element_2 self))))))

(event EventTiirScenarioShutdown
  (Development|PrintString "Tiir Scenario Shutdown" false true "(R=0.000000,G=0.660000,B=1.000000,A=1.000000)" 6e+01)
  (if (Class|TiirUniverse|IsGameOver)
    (Development|PrintString "Tiir Game Over" false true "(R=0.000000,G=0.660000,B=1.000000,A=1.000000)" 6e+01)
    (if (Class|TiirUniverse|WasMissionSuccesful)
      (CallFunction|SetUsePersistentFleet true))
    (CallFunction|SubmitCampaignResults)))

(event EventTiirScenarioStartup
  (Development|PrintString "Tiir Scenario Startup" false true "(R=0.000000,G=0.660000,B=1.000000,A=1.000000)" 6e+01)
  (if (not (Variables|Default|GetInAnimatic)) ; Is an animatic currently active?
    (bind _animaticwidget (CallFunction|StartupCampaign))
    (Variables|Default|SetPassedStartupCampaign true)
    (Utilities|IsValid _animaticwidget
      (:Is%20Valid
        (Variables|Default|SetInAnimatic true)
        (EventDispatchers|BindEventtoAnimaticCompletedEvent _animaticwidget (delegate Custom|PostAnimatic)))
      (:Is%20Not%20Valid
        (Class|TiirUtilities|TiirDelay 0.2)
        (Default|CallOpeningAnimaticComplete)
        (bind _objects (Class|TiirUtilities|GetTiirScriptswithInterface "/Game/Assets/Blueprints/Campaign/BPI_CampaignFlow.BPI_CampaignFlow_C"))
        (for _array_element _objects
          (bind _type (Class|BPICampaignFlow|TiirFleetSpawnType(Message) _array_element))
          (Variables|Default|SetFleetSpawnType _type))
        (CallFunction|LoadStartingFleets (Variables|Default|GetFleetSpawnType) false "ParadeHyperspace")
        (for _array_element_2 _objects
          (Class|BPICampaignFlow|TiirPostAnimatic(Message) _array_element_2 self))))))

(fn DebugPrintStartingFleet
  (params (ScenarioFleetConfig :type Scenario%20Fleet%20Config%20Structure%20%28by%20ref%29))
  (bind _units (Utilities|Struct|BreakScenarioFleetConfig ScenarioFleetConfig))
  (bind (_mothership _items) (Utilities|Struct|BreakScenarioShipConfig _units))
  (bind (_hold _type) (Utilities|Struct|BreakScenarioShipItem _mothership))
  (Utilities|FlowControl|Sequence
    (:then_0
      (Development|PrintString (Utilities|String|Append "Saving Mothership:  " _type) false true "(R=1.000000,G=0.000000,B=0.026037,A=1.000000)" 6e+01))
    (:then_1
      (for _array_element _hold
        (Development|PrintString (Utilities|String|Append "Saving MS Hold Ship:  " (.type _array_element)) false true "(R=1.000000,G=0.000000,B=0.026037,A=1.000000)" 6e+01)))
    (:then_2
      (for _array_element_2 _items
        (Development|PrintString (Utilities|String|Append "Saving Ship: " (.type _array_element_2)) false true "(R=1.000000,G=0.000000,B=0.026037,A=1.000000)" 6e+01)
        (for _array_element_3 (.hold _array_element_2)
          (Development|PrintString (Utilities|String|Append "Saving in Hold: " (.type _array_element_3)) false true "(R=1.000000,G=0.000000,B=0.026037,A=1.000000)" 6e+01))))))

(fn SubmitCampaignResults
  (bind _persistentfleetsavegame (Variables|Default|GetPersistentFleetSaveGame))
  (bind _playerstarts (Variables|Default|GetPlayerStarts))
  (Utilities|FlowControl|Sequence
    (:then_0
      (if (and (Class|TiirUniverse|IsGameOver) (Class|TiirUniverse|WasMissionSuccesful))
        (bind _returnvalue (Class|TiirUtilities|GetCurrentFleet (.Player (Class|TiirPlayerFunctionLibrary|GetPlayerfromIndex))))
        (LocalVariables|SetFleetToProceedWith _returnvalue)
        (else
          (Utilities|IsValid _persistentfleetsavegame
            (:Is%20Valid
              (LocalVariables|SetFleetToProceedWith (Variables|/Game/Assets/Gameplay/BP_PersistentFleetSaveGame.BP_PersistentFleetSaveGame_C|GetFleet _persistentfleetsavegame)))
            (:Is%20Not%20Valid
              (if (Utilities|Array|IsValidIndex _playerstarts)
                (LocalVariables|SetFleetToProceedWith (Class|TiirUtilities|ConverttoFleetConfig (Class|RTSPlayerStart|GetStartingFleetData (Utilities|Array|Get(acopy) _playerstarts))))))))))
    (:then_1
      (CallFunction|DebugPrintStartingFleet (LocalVariables|GetFleetToProceedWith)))
    (:then_2
      (if (Class|TiirUniverse|WasMissionSuccesful)
        (bind _returnvalue_2 (Game|GetCurrentLevelName true))
        (bind _asbp_raven_game_instance (Utilities|Casting|CastToBP_RavenGameInstance (Game|GetGameInstance)))
        (Default|SaveCampaignProgress _asbp_raven_game_instance _returnvalue_2 true)
        (bind (_returnvalue_3 _reachedend) (CallFunction|FindNextLevelName))
        (CallFunction|SubmitCampaignResultEvent (LocalVariables|GetFleetToProceedWith) _returnvalue_3 _reachedend)
        (else
          ;[1 1 1] To do: remove platform check once PS5 functionality is ready. Everything should be routed through RavenHUD to the proper destination.
          (Class|PlatformInfoSubsystem|CheckIsPlatformasExec (|PlatformInfoSubsystem) "PS5"
            (:True
              (bind _returnvalue_4 (Game|GetCurrentLevelName true))
              (CallFunction|SubmitCampaignResultEvent (LocalVariables|GetFleetToProceedWith) (Utilities|String|StringToName _returnvalue_4) false))
            (:False
              (bind _asraven_player_controller (Utilities|Casting|CastToRavenPlayerController (Game|GetPlayerController 0)))
              (Default|ShowMissionFailedHudPanel (Variables|/Game/Assets/Gameplay/RavenPlayerController.RavenPlayerController_C|GetRavenHUD _asraven_player_controller)))))))))

(fn LoadStartingFleets
  (params (SpawnTypes :type EPersistentFleetSpawnTypes%20Enum :default "FullFleet") (override%20Spawn%20Behaviour :type Boolean) (new%20Spawn%20Behaviour :type EPersistentFleetBehaviour%20Enum :default "ParadeHyperspace"))
  (bind _returnvalue (Game|GetGameMode))
  ;[1 1 1] Only restrict research during the campaign
  (Utilities|Casting|CastToBP_MultiplayerRavenGameMode _returnvalue
    (:then
      _)
    (:CastFailed
      (Utilities|Casting|CastToBP_AIDemoGameMode _returnvalue
        (:then
          _)
        (:CastFailed
          (Utilities|Casting|CastToBP_PvEMole_GameMode _returnvalue)
          (for _index (range 0 1)
            (Class|TiirResearchFunctionLibrary|RestrictResearchTechTreeforPlayer _index true))))))
  (Variables|Default|SetPersistentFleetSaveGame 0)
  (bind _returnvalue_2 (Game|GetCurrentLevelName true))
  (Utilities|PrintStringwithPrefix "New Behaviour" (Utilities|String|EnumtoString new%20Spawn%20Behaviour) true 3.0
    (:Out
      (bind _output_get (LocalVariables|SetPersistentFleetName _returnvalue_2))
      (bind _returnvalue_3 (Class|RTSSaveGameSubsystem|LoadProfileSave (Subsystems|GetRTSSaveGameSubsystem)))
      (bind _returnvalue_4 (Class|ProfileSaveGame|HasPersistentFleetforLevel _returnvalue_3 _output_get))
      (bind _usepersistentfleet (CallFunction|GetUsePersistentFleet))
      (if (and _usepersistentfleet _returnvalue_4)
        (CallFunction|LoadPersistentFleet (LocalVariables|GetPersistentFleetName) SpawnTypes override%20Spawn%20Behaviour new%20Spawn%20Behaviour)
        (else
          (CallFunction|LoadDefaultFleet "" SpawnTypes override%20Spawn%20Behaviour new%20Spawn%20Behaviour)))
      (CallFunction|SetDifficultyModifiers))))

(fn StartupCampaign
  ;[1 1 1] Copy Profile Difficulty Settings to Scenario Parameters
  (bind _returnvalue (Class|RTSSaveGameSubsystem|LoadProfileSave (Subsystems|GetRTSSaveGameSubsystem)))
  (Variables|Default|SetSelectedDifficultyPreset (Variables|/Script/Raven.SaveCampaignProgress|GetSelectedDifficultyPreset (Variables|/Script/Raven.ProfileSaveGame|GetCampaignProgress _returnvalue)))
  (Variables|Default|SetCampaignDifficulty_Custom (Variables|/Script/Raven.SaveCampaignProgress|GetCampaignDifficulty_Custom (Variables|/Script/Raven.ProfileSaveGame|GetCampaignProgress _returnvalue)))
  (Utilities|FlowControl|Sequence
    (:then_0
      (bind _returnvalue_2 (Game|GetCurrentLevelName true))
      (bind _output_get (LocalVariables|SetCurrentLevelLocal (Utilities|String|StringToName _returnvalue_2)))
      (bind _returnvalue_3 (Utilities|GetDataTableRow (Variables|Default|GetCampaignMissionData) _output_get)
        (:then
          (Utilities|IsValid (.IntroCutscene (Utilities|Struct|BreakPrototypeLevelData _returnvalue_3))
            (:Is%20Valid
              (bind _output_get_2 (Variables|ScenarioParameters|SetStayBlankAtStart (.KeepUIHiddenOnStart (Utilities|Struct|BreakPrototypeLevelData _returnvalue_3))))
              (if _output_get_2
                (CallFunction|BlankGameplayScreen))
              (for _index (range 0 1)
                (bind _asraven_player_controller (Utilities|Casting|CastToRavenPlayerController (Class|GameplayStatics|GetPlayerControllerfromID _index)))
                (Default|LetterBox _asraven_player_controller true true false 2.0)
                (Default|HideHUD _asraven_player_controller true)
                (bind _returnvalue_4 (UserInterface|CreateWidget "/Game/Movies/AnimaticPlayerWidget.AnimaticPlayerWidget_C" _asraven_player_controller))
                (bind _output_get_3 (LocalVariables|SetActiveAnimaticLocal _returnvalue_4))
                (UserInterface|Viewport|AddtoViewport _output_get_3 0)
                (Default|PlayCutscene _output_get_3 (.IntroCutscene (Utilities|Struct|BreakPrototypeLevelData _returnvalue_3)))))))))
    (:then_1
      (return (LocalVariables|GetActiveAnimaticLocal)))))

(fn FindNextLevelName
  (bind _campaignmissiondata (Variables|Default|GetCampaignMissionData))
  (Utilities|FlowControl|Sequence
    (:then_0
      (bind _returnvalue (Game|GetCurrentLevelName true))
      (LocalVariables|SetDesiredLevel (Utilities|String|StringToName _returnvalue)))
    (:then_1
      (bind _outrownames (DataTable|GetDataTableRowNames _campaignmissiondata))
      (bind _output_get (LocalVariables|SetCampaignLevelIndex (Utilities|Array|FindItem _outrownames (LocalVariables|GetDesiredLevel))))
      (bind _output_get_2 (LocalVariables|SetNextLevelIndex -1))
      (while (Math|Boolean|ANDBoolean (< _output_get_2 0) (> _output_get -1) (< _output_get (Utilities|Array|Length _outrownames)))
        (bind _result (Math|Integer|IncrementInt (LocalVariables|GetCampaignLevelIndex))
          (:%20%20
            (if (Utilities|Array|IsValidIndex _outrownames _result)
              (bind _returnvalue_2 (Utilities|GetDataTableRow _campaignmissiondata (Utilities|Array|Get(acopy) _outrownames _result))
                (:then
                  (if (.Enabled (Utilities|Struct|BreakPrototypeLevelData _returnvalue_2))
                    (LocalVariables|SetNextLevelIndex _result)
                    (LocalVariables|SetDesiredLevel (Utilities|Array|Get(acopy) _outrownames _result))))))))))
    (:then_2
      (return (LocalVariables|GetDesiredLevel) (== (LocalVariables|GetNextLevelIndex) -1)))))

(fn ConstructionScript)

(fn LoadStartingFleetforPlayer
  (params (PlayerStart :type RTS%20Player%20Parameters%20Object%20Reference) (SpawnTypes :type EPersistentFleetSpawnTypes%20Enum :default "FullFleet") (override%20Spawn%20Behaviour :type Boolean) (NewSpawnBehaviour :type EPersistentFleetBehaviour%20Enum :default "ParadeHyperspace"))
  (bind _commanderassignment (Variables|/Script/Raven.RTSPlayerParameters|GetCommanderAssignment PlayerStart))
  (bind _player (Class|TiirPlayerFunctionLibrary|GetPlayerfromIndex (.commanderid _commanderassignment)))
  (bind _returnvalue (Class|TiirUtilities|ConverttoFleetConfig (.startingfleet _commanderassignment)))
  (Utilities|IsValid (.startingfleet _commanderassignment)
    (:Is%20Valid
      (CallFunction|LoadSimFleetforPlayerStart _player _returnvalue (Utilities|Array|Get(acopy) (Variables|Default|GetPlayerStarts) (.playerstartindex _commanderassignment)) SpawnTypes 1.0 override%20Spawn%20Behaviour NewSpawnBehaviour)
      (Class|TiirUtilities|LoadFleetResources _player _returnvalue))))

(fn LoadSimFleetforPlayerStart
  (params (Commander :type Tiir%20Commander%20Structure%20%28by%20ref%29) (Fleet :type Scenario%20Fleet%20Config%20Structure%20%28by%20ref%29) (PlayerStart :type RTS%20Player%20Start%20Object%20Reference) (SpawnTypes :type EPersistentFleetSpawnTypes%20Enum :default "FullFleet") (FleetHealPercent :type Float%20%28single-precision%29) (override%20Spawn%20Behaviour :type Boolean) (NewSpawnBehaviour :type EPersistentFleetBehaviour%20Enum :default "ParadeHyperspace"))
  (Utilities|FlowControl|Sequence
    (:then_0
      (bind _asbp_campaign_player_start (Utilities|Casting|CastToBP_Campaign_PlayerStart PlayerStart))
      (LocalVariables|SetFleetLoadBehaviour (select override%20Spawn%20Behaviour NewSpawnBehaviour (Variables|/Game/Assets/Blueprints/Campaign/BP_Campaign_PlayerStart.BP_Campaign_PlayerStart_C|GetStartingFleetBehaviour _asbp_campaign_player_start)))
      (LocalVariables|SetAutolaunchBehaviour (Variables|/Game/Assets/Blueprints/Campaign/BP_Campaign_PlayerStart.BP_Campaign_PlayerStart_C|GetStartingFleetAutolaunchBehaviour _asbp_campaign_player_start)))
    (:then_1
      (bind _returnvalue (Class|RTSPlayerStart|GetFleetStartingPosition PlayerStart))
      (Class|TiirUtilities|LoadFleetat Commander Fleet _returnvalue (LocalVariables|GetFleetLoadBehaviour) (LocalVariables|GetAutolaunchBehaviour) SpawnTypes FleetHealPercent))))

(fn GetFleetHealPercentage
  (bind _value (CallFunction|GetFleetRepairScale))
  (return _value))

(fn GetCampaignDifficultySettings
  (bind _selecteddifficultypreset (Variables|Default|GetSelectedDifficultyPreset))
  (bind _asbp_raven_game_instance (Utilities|Casting|CastToBP_RavenGameInstance (Game|GetGameInstance)))
  (bind _campaignprogress (Variables|/Game/Assets/Gameplay/BP_RavenGameInstance.BP_RavenGameInstance_C|GetCampaignProgress _asbp_raven_game_instance)
    (:then
      (if (Variables|Default|GetPassedStartupCampaign) ; This function may be called before we have cached SelectedDifficultyPreset or SelectedDifficultyCustom
        (if (Utilities|Enum|Equal(Enum) _selecteddifficultypreset "Custom")
          (return (Variables|Default|GetCampaignDifficulty_Custom))
          (else
            (bind _difficultysettings (Default|GetDifficultySettingsforPreset _campaignprogress _selecteddifficultypreset))
            (return _difficultysettings)))
        (else
          (return (Default|GetDifficultySettingsforSelectedPreset _campaignprogress)))))
    (:else
      (Development|PrintText "Error! Missing global campaign progress"))))

(fn GetLevelParameters
  (params (LevelName :type String))
  (bind _returnvalue (Utilities|GetDataTableRow (Variables|Default|GetCampaignMissionData) (Utilities|String|StringToName LevelName))
    (:then
      (return _returnvalue))
    (:RowNotFound
      (return ""))))

(fn CreateMoviePaths
  (params (MediaSources :type Array%20of%20File%20Media%20Source%20Object%20References))
  (for _array_element MediaSources
    (Utilities|Array|Add (LocalVariables|GetLocalMoviePaths) (Utilities|String|Append "Loading/" (Utilities|GetObjectName _array_element))))
  (return (LocalVariables|GetLocalMoviePaths)))

(fn LoadDefaultFleet
  (params (Persistent%20Fleet%20Name :type String) (Spawn%20Types :type EPersistentFleetSpawnTypes%20Enum :default "FullFleet") (override%20Spawn%20Behaviour :type Boolean) (NewSpawn%20Behaviour :type EPersistentFleetBehaviour%20Enum :default "ParadeHyperspace"))
  (CallFunction|DeletePersistentFleetSave Persistent%20Fleet%20Name)
  (for _array_element (Variables|Default|GetPlayers)
    (CallFunction|LoadStartingFleetforPlayer _array_element Spawn%20Types override%20Spawn%20Behaviour NewSpawn%20Behaviour))
  (for _array_element_2 (Variables|Default|GetAIPlayers)
    (CallFunction|LoadStartingFleetforPlayer _array_element_2 Spawn%20Types override%20Spawn%20Behaviour NewSpawn%20Behaviour)))

(fn LoadPersistentFleet
  (params (PersistentFleetName :type String) (SpawnTypes :type EPersistentFleetSpawnTypes%20Enum :default "FullFleet") (Override%20Spawn%20Behaviour :type Boolean) (New%20Spawn%20Behaviour :type EPersistentFleetBehaviour%20Enum :default "ParadeHyperspace") (CommanderID :type Integer))
  (bind _returnvalue (Class|RTSSaveGameSubsystem|LoadProfileSave (Subsystems|GetRTSSaveGameSubsystem)))
  (bind _returnvalue_2 (Class|ProfileSaveGame|GetPersistentFleetforLevel _returnvalue PersistentFleetName))
  (switch Utilities|FlowControl|Switch|SwitchonEPersistentFleetSpawnTypes SpawnTypes
    (:FullFleet
      _)
    (:Motherships
      (bind _output_get (Variables|Default|SetLoadedPersistentMotherships true))
      (if (and _output_get (stale _output_get_2)) :!label _label
        _
        (else
          _)))
    (:NonMotherships
      (bind _output_get_2 (Variables|Default|SetLoadedPersistentNonMotherships true))
      (goto _label)))
  (bind _asbp_persistent_fleet_save_game (Utilities|Casting|CastToBP_PersistentFleetSaveGame _returnvalue_2))
  (bind _output_get_3 (Variables|Default|SetPersistentFleetSaveGame _asbp_persistent_fleet_save_game))
  (LocalVariables|SetPersistentFleet (Variables|/Game/Assets/Gameplay/BP_PersistentFleetSaveGame.BP_PersistentFleetSaveGame_C|GetFleet _output_get_3))
  (for _index (range 0 1)
    (bind _asraven_player_controller (Utilities|Casting|CastToRavenPlayerController (Class|GameplayStatics|GetPlayerControllerfromID CommanderID)))
    (Class|SimulationProxy|SetSimPersistentFleetSave (Class|RTSPlayerController|GetSimulationProxy _asraven_player_controller) (Variables|/Game/Assets/Gameplay/BP_PersistentFleetSaveGame.BP_PersistentFleetSaveGame_C|GetSavedEntities _output_get_3))
    (bind _asbp_campaign_player_start (Utilities|Casting|CastToBP_Campaign_PlayerStart (Utilities|Array|Get(acopy) (Variables|Default|GetPlayerStarts) CommanderID)))
    (if (== CommanderID 0)
      (LocalVariables|SetFirstPlayerStart _asbp_campaign_player_start)
      (else
        (LocalVariables|SetSecondPlayerStart _asbp_campaign_player_start)))
    (Variables|/Game/Assets/Blueprints/Campaign/BP_Campaign_PlayerStart.BP_Campaign_PlayerStart_C|SetMatchToPersistentFleet (Utilities|Select :Index CommanderID :Option%200 (LocalVariables|GetFirstPlayerStart) :Option%201 (LocalVariables|GetSecondPlayerStart)) (.startingfleet (Variables|/Script/Raven.RTSPlayerParameters|GetCommanderAssignment (Utilities|Array|Get(acopy) (Class|RTSScenarioParameters|GetPlayers) CommanderID))))
    (if (or (Utilities|Enum|Equal(Enum) SpawnTypes "FullFleet") (Utilities|Enum|Equal(Enum) SpawnTypes "Motherships"))
      (Class|TiirUtilities|LoadFleetResources (.Player (Class|TiirPlayerFunctionLibrary|GetPlayerfromIndex CommanderID)) (LocalVariables|GetPersistentFleet)))
    (Utilities|IsValid (Variables|/Game/Assets/Blueprints/Campaign/BP_Campaign_PlayerStart.BP_Campaign_PlayerStart_C|GetMatchToPersistentFleet (Utilities|Select :Index CommanderID :Option%200 (LocalVariables|GetFirstPlayerStart) :Option%201 (LocalVariables|GetSecondPlayerStart)))
      (:Is%20Valid
        (if (Variables|Default|GetMergePersistentFleet)
          (CallFunction|LoadSimFleetforPlayerStart (.Player (Class|TiirPlayerFunctionLibrary|GetPlayerfromIndex CommanderID)) (Class|TiirUtilities|MatchFleetConfigs (LocalVariables|GetPersistentFleet) (Class|TiirUtilities|ConverttoFleetConfig (Variables|/Game/Assets/Blueprints/Campaign/BP_Campaign_PlayerStart.BP_Campaign_PlayerStart_C|GetMatchToPersistentFleet (Utilities|Select :Index CommanderID :Option%200 (LocalVariables|GetFirstPlayerStart) :Option%201 (LocalVariables|GetSecondPlayerStart))))) (Utilities|Select :Index CommanderID :Option%200 (LocalVariables|GetFirstPlayerStart) :Option%201 (LocalVariables|GetSecondPlayerStart)) SpawnTypes (CallFunction|GetFleetHealPercentage) (LocalVariables|Getoverride%20Spawn%20Behaviour) (LocalVariables|Getnew%20Spawn%20Behaviour))
          (else
            (CallFunction|LoadSimFleetforPlayerStart (.Player (Class|TiirPlayerFunctionLibrary|GetPlayerfromIndex CommanderID)) (Class|TiirUtilities|MatchFleetResearch (LocalVariables|GetPersistentFleet) (Class|TiirUtilities|ConverttoFleetConfig (Variables|/Game/Assets/Blueprints/Campaign/BP_Campaign_PlayerStart.BP_Campaign_PlayerStart_C|GetMatchToPersistentFleet (Utilities|Select :Index CommanderID :Option%200 (LocalVariables|GetFirstPlayerStart) :Option%201 (LocalVariables|GetSecondPlayerStart))))) (Utilities|Select :Index CommanderID :Option%200 (LocalVariables|GetFirstPlayerStart) :Option%201 (LocalVariables|GetSecondPlayerStart)) SpawnTypes (CallFunction|GetFleetHealPercentage) (LocalVariables|Getoverride%20Spawn%20Behaviour) (LocalVariables|Getnew%20Spawn%20Behaviour) :!label _label_2))))
      (:Is%20Not%20Valid
        (goto _label_2)))
    (Utilities|IsValid (Variables|/Game/Assets/Blueprints/Campaign/BP_Campaign_PlayerStart.BP_Campaign_PlayerStart_C|GetAddToPersistentFleet (Utilities|Select :Index CommanderID :Option%200 (LocalVariables|GetFirstPlayerStart) :Option%201 (LocalVariables|GetSecondPlayerStart)))
      (:Is%20Valid
        (CallFunction|LoadSimFleetforPlayerStart (.Player (Class|TiirPlayerFunctionLibrary|GetPlayerfromIndex CommanderID)) (Class|TiirUtilities|ConverttoFleetConfig (Variables|/Game/Assets/Blueprints/Campaign/BP_Campaign_PlayerStart.BP_Campaign_PlayerStart_C|GetAddToPersistentFleet (Utilities|Select :Index CommanderID :Option%200 (LocalVariables|GetFirstPlayerStart) :Option%201 (LocalVariables|GetSecondPlayerStart)))) (Utilities|Select :Index CommanderID :Option%200 (LocalVariables|GetFirstPlayerStart) :Option%201 (LocalVariables|GetSecondPlayerStart)) SpawnTypes (CallFunction|GetFleetHealPercentage) (LocalVariables|Getoverride%20Spawn%20Behaviour) (LocalVariables|Getnew%20Spawn%20Behaviour))))))

(fn GetUsePersistentFleet
  (bind _asbp_raven_game_instance (Utilities|Casting|CastToBP_RavenGameInstance (Game|GetGameInstance)))
  (bind _campaignprogress (Variables|/Game/Assets/Gameplay/BP_RavenGameInstance.BP_RavenGameInstance_C|GetCampaignProgress _asbp_raven_game_instance)
    (:then
      (bind _usepersistentfleet (Default|GetUsePersistentFleet _campaignprogress))
      (return _usepersistentfleet))
    (:else)))

(fn SetUsePersistentFleet
  (params (UsePersistentFleet :type Boolean))
  (bind _asbp_raven_game_instance (Utilities|Casting|CastToBP_RavenGameInstance (Game|GetGameInstance)))
  (bind _campaignprogress (Variables|/Game/Assets/Gameplay/BP_RavenGameInstance.BP_RavenGameInstance_C|GetCampaignProgress _asbp_raven_game_instance)
    (:then
      (Default|SetUsePersistentFleet _campaignprogress UsePersistentFleet)
      (bind _asbp_raven_game_instance_2 (Utilities|Casting|CastToBP_RavenGameInstance (Game|GetGameInstance)))
      (Default|SaveCampaignProgress _asbp_raven_game_instance_2 "" true)
      (return))
    (:else)))

(fn DeletePersistentFleetSave
  (params (PersistentFleetName :type String))
  (bind _returnvalue (Subsystems|GetRTSSaveGameSubsystem))
  (if (not (Class|DebugSettingsFunctionLibrary|ForceMaintainFleetSave))
    (bind _returnvalue_2 (Class|RTSSaveGameSubsystem|LoadProfileSave _returnvalue))
    (Class|ProfileSaveGame|RemovePersistentFleetforLevel _returnvalue_2 PersistentFleetName)
    (Class|RTSSaveGameSubsystem|StoreProfileSave _returnvalue)
    (return)))

(fn SetDifficultyModifiers
  (Class|TiirDifficulty|SetDifficulty 0 (CallFunction|GetCampaignDifficultySettings)))

(fn GetDifficultyPreset
  (bind _asbp_raven_game_instance (Utilities|Casting|CastToBP_RavenGameInstance (Game|GetGameInstance)))
  (bind _campaignprogress (Variables|/Game/Assets/Gameplay/BP_RavenGameInstance.BP_RavenGameInstance_C|GetCampaignProgress _asbp_raven_game_instance)
    (:then
      (if (Variables|Default|GetPassedStartupCampaign) ; This function may be called before we have cached SelectedDifficultyPreset or SelectedDifficultyCustom
        (return (Variables|Default|GetSelectedDifficultyPreset))
        (else
          (return (Variables|/Script/Raven.SaveCampaignProgress|GetSelectedDifficultyPreset _campaignprogress)))))
    (:else
      (Development|PrintText "Error! Missing global campaign progress"))))