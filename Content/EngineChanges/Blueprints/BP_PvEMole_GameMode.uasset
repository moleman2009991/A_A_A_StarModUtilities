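; PvE Mole game mode Blueprint that handles co-op mission end, level transitions and session exit.
; At mission end it sends a co-op level change through every session beacon client when transitions are enabled and a next level is set, otherwise deferring to the parent.
; Beacon clients also receive the hyperspace button prompt.
; Reconnection resets time dilation before connecting, while timeouts leave the lobby, clear quick play and exit to menu.
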(event EventMultiplayerEndGame
  (params (WasMissionSuccessful :type Boolean))
  (if (Variables|Default|GetTransitonLevels?_0)
    (if (Utilities|Name|Equal(Name) (Variables|Default|GetNext%20Level_0) "None")
      (|CallParentFunction WasMissionSuccessful :!label _label)
      (else
        (Variables|Default|SetIsMovingToNextCoopLevel true)
        (bind _outactors (Actor|GetAllActorsOfClass "/Game/Assets/Gameplay/RavenSessionBeaconClient.RavenSessionBeaconClient_C"))
        (for _array_element _outactors
          (Default|SubmitChangeLevel _array_element (Variables|Default|GetNext%20Level_0) true))))
    (else
      (goto _label))))

(event EventMultiplayerShowHyperspace
  (bind _outactors (Actor|GetAllActorsOfClass "/Game/Assets/Gameplay/RavenSessionBeaconClient.RavenSessionBeaconClient_C"))
  (for _array_element _outactors
    (Default|ReceiveShowHyperspaceButton _array_element)))

(event EventStartAttemptReconnection
  (params (Dest%20Options :type String))
  (Utilities|Time|SetGlobalTimeDilation 1.0)
  (Class|RTSGameMode|AttemptSessionConnection Dest%20Options "EnteringGame"))

(event EventOnTimeOut
  (CallFunction|PrintLobbyStateDebugString -1)
  (CallFunction|ExittoMenu))

(event EventExittoMenu
  (bind _returnvalue (Subsystems|GetRavenOnlineServices))
  (|LeaveLocalRavenLobby _returnvalue (Game|GetPlayerController 0) true
    (:OnComplete
      (Class|RavenOnlineServices|SetQuickPlay _returnvalue false)
      (CallFunction|ExittoMainMenu))))

(fn ConstructionScript)