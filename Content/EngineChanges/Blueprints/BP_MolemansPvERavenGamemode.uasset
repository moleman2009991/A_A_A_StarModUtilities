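; Game mode for PvE multiplayer that handles mission end, reconnection and exit to the main menu.
; On mission end the host leaves the online match and, given PvE scenario parameters, sends an end-game order and notifies every beacon client whether another level follows.
; The end-game check holds off during host migration or missing session state.
; Helper functions lower the resource multiplier by difficulty and apply it to map resource spawners.
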(event Custom|OnTimeOut
  (CallFunction|ExittoMenu))

(event Custom|StartAttemptReconnection
  (params (Dest%20Options :type String))
  (Utilities|Time|SetGlobalTimeDilation 1.0)
  (Class|RTSGameMode|AttemptSessionConnection Dest%20Options "EnteringGame"))

(event Custom|ExitToMenu
  (bind _returnvalue (Subsystems|GetRavenOnlineServices))
  (|LeaveLocalRavenLobby _returnvalue (Game|GetPlayerController 0) true
    (:OnComplete
      (Class|RavenOnlineServices|SetQuickPlay _returnvalue false)
      (CallFunction|ExittoMainMenu))))

(event Custom|MultiplayerEndGame
  (params (WasMissionSuccessful :type Boolean))
  (Variables|Default|SetLocalWasMissionSuccessful WasMissionSuccessful)
  (Development|PrintString "BP_MultiplayerRavenGameMode MultiplayerEndGame")
  ;[1 1 1] VTS|PS5 call the leave match after the game finished (on the host side)
  (Class|RavenOnlineServices|LeaveCurrentMatch (Subsystems|GetRavenOnlineServices) "Finished")
  (bind _asbp_pv_edemo_scenario_parameters (Utilities|Casting|CastToBP_PvEDemo_ScenarioParameters (Variables|/Script/Raven.RTSSessionBeaconState|GetParameters (Variables|/Script/Raven.RTSSessionBeaconClient|GetSessionState (Variables|Default|GetSessionClient))))
    (:then
      (bind _haslevel (Default|HasNextMultiplayerLevel _asbp_pv_edemo_scenario_parameters))
      (Variables|Default|SetIsMovingToNextCoopLevel _haslevel)
      (bind _asraven_player_controller (Utilities|Casting|CastToRavenPlayerController (Game|GetPlayerController 0)))
      (bind _returnvalue (Game|ConstructObjectfromClass "/Game/Assets/Blueprints/Orders/BPO_InvokeCommandEndGame.BPO_InvokeCommandEndGame_C" _asraven_player_controller))
      (Variables|/Game/Assets/Blueprints/Orders/BPO_InvokeCommandEndGame.BPO_InvokeCommandEndGame_C|SetMissionSuccessful _returnvalue (Variables|Default|GetLocalWasMissionSuccessful))
      (Class|RTSPlayerUnitOrderComponent|SendOrder (Variables|/Script/Raven.RTSPlayerController|GetUnitOrderComponent _asraven_player_controller) (Class|SimOrderFactory|MakeScriptActionOrder (Variables|/Script/Raven.RTSPlayerController|GetSimPlayer _asraven_player_controller) _returnvalue))
      (Development|PrintString "Calling ReceiveEndGame for all clients")
      (bind _outactors (Actor|GetAllActorsOfClass "/Game/Assets/Gameplay/RavenSessionBeaconClient.RavenSessionBeaconClient_C"))
      (for _array_element _outactors
        (Development|PrintText (Utilities|Text|FormatText "Firing ReceiveEndGame for client: {0}" (Utilities|GetDisplayName _array_element)))
        (Default|ReceiveEndGame _array_element (Variables|Default|GetLocalWasMissionSuccessful) (Variables|Default|GetIsMovingToNextCoopLevel))))
    (:CastFailed
      (Variables|Default|SetIsMovingToNextCoopLevel false))))

(event Custom|MultiplayerShowHyperspace
  (bind _outactors (Actor|GetAllActorsOfClass "/Game/Assets/Gameplay/RavenSessionBeaconClient.RavenSessionBeaconClient_C"))
  (for _array_element _outactors
    (Default|ReceiveShowHyperspaceButton _array_element)))

(fn ConstructionScript)

(fn ShouldEndMultiplayerinGameState
  (bind _sessionclient (Variables|Default|GetSessionClient))
  (bind _sessionstate (Variables|/Script/Raven.RTSSessionBeaconClient|GetSessionState _sessionclient))
  (bind _returnvalue (Class|RTSNetworkManager|GetIsMigratingHostorPreloadingorResuming (Variables|/Script/Raven.RTSGameMode|GetNetworkManager (.AsRaven%20Game%20Mode (Utilities|Casting|CastToRavenGameMode (Game|GetGameMode))))))
  (if _returnvalue
    (return false) ; If we're migrating hosts, don't end the game
    (else
      (Utilities|IsValid _sessionstate
        (:Is%20Valid
          (return (not (Class|RTSSessionBeaconState|HasatLeastPlayersActive _sessionstate 1))) ; The only time we want to end the game is if hosts are not migrating and there are no active players left.
        )
        (:Is%20Not%20Valid
          (return false) ; After a host migration it takes some time for the SessionState to be replicated,\nso we need to avoid ending the game in that case too.
        )))))

(fn InitMapResources
  (bind _game_instance (CallFunction|GetRavenGameInstancePure))
  (bind _multiplayerscenarioparameters (Variables|/Game/Assets/Gameplay/BP_RavenGameInstance.BP_RavenGameInstance_C|GetMultiplayerScenarioParameters _game_instance))
  (bind _resourcemultiplier (Variables|/Script/Raven.MultiplayerRavenScenarioParameters|GetResourceMultiplier _multiplayerscenarioparameters))
  (Development|PrintString (Utilities|String|Append "Resource Multiplier Is : " (Utilities|String|ToString(Float) _resourcemultiplier)))
  (if (!= 1.0 _resourcemultiplier)
    (bind _outactors (Actor|GetAllActorsOfClass "/Script/RavenSimulation.TiirResourceSpawner"))
    (for _array_element _outactors
      (Variables|/Script/RavenSimulation.TiirResourceSpawner|SetResourceModifier _array_element (* (Variables|/Script/RavenSimulation.TiirResourceSpawner|GetResourceModifier _array_element) _resourcemultiplier)))))

(fn WGsMapResourceReduction
  (bind _game_instance (CallFunction|GetRavenGameInstancePure))
  (bind _multiplayerscenarioparameters (Variables|/Game/Assets/Gameplay/BP_RavenGameInstance.BP_RavenGameInstance_C|GetMultiplayerScenarioParameters _game_instance))
  (switch Utilities|FlowControl|Switch|SwitchonEMultiplayerGameDifficulty (Variables|/Script/Raven.MultiplayerRavenScenarioParameters|GetRunDifficulty _multiplayerscenarioparameters)
    (:Diff2
      (Variables|/Script/Raven.MultiplayerRavenScenarioParameters|SetResourceMultiplier _multiplayerscenarioparameters 0.9 :!label _label))
    (:Diff3
      (goto _label))
    (:Diff4
      (goto _label))
    (:Diff5
      (goto _label))
    (:Diff6
      (goto _label))
    (:Diff7
      (goto _label))
    (:Diff8
      (Variables|/Script/Raven.MultiplayerRavenScenarioParameters|SetResourceMultiplier _multiplayerscenarioparameters 0.8 :!label _label_2))
    (:Diff9
      (goto _label_2))
    (:Diff10
      (goto _label_2))))