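; Camera rig actor that follows a focus actor and aims its camera at it.
; A looping 0.4-second task calls TrackActor, which uses a task-based delta timer macro to lerp the rig toward that actor's location.
; Shared utility macros apply zoom, offsets, arm rotation, lens settings and look-at rotation from the construction script and UpdateCameraPositon.
; UpdateCameraPositon can also move the rig, and SetFocusActor changes the target.
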(event Custom|Update%20Camera%20Positon
  (params (bSweep :type Boolean) (bTeleport :type Boolean) (Update%20Location :type Boolean) (New%20Location :type Vector))
  (bind (_zoom _x_offset _y_offset _roll _pitch _yaw _aspect_ratio _field_of_view) (Utilities|Utility-GetCameraSettings))
  (if Update%20Location
    (Transformation|SetActorLocation New%20Location bSweep bTeleport))
  (Utilities|Utility-SetCameraSettings (Variables|Default|GetCamera) (Variables|Default|GetSpringArm) (Variables|Controls|GetActor%20to%20Focus) _zoom _x_offset _y_offset _roll _pitch _yaw _aspect_ratio _field_of_view bSweep bTeleport))

(event Custom|Track%20Actor
  (bind _actor_to_focus (Variables|Controls|GetActor%20to%20Focus))
  (Utilities|IsValid _actor_to_focus
    (:Is%20Valid
      (bind _alpha_ (Utilities|Utility-DeltaTimer 0.2)
        (:execute
          (Transformation|SetActorLocation (Math|Vector|Lerp(Vector) (Transformation|GetActorLocation self) (Transformation|GetActorLocation _actor_to_focus) _alpha_) false false))))))

(event Custom|Set%20Focus%20Actor
  (params (Actor%20to%20Focus :type Actor%20Object%20Reference))
  (Variables|Controls|SetActor%20to%20Focus Actor%20to%20Focus))

(event EventBeginPlay
  (|TaskTimer :bLooping true :Time 0.4
    (:Elapsed
      (CallFunction|TrackActor))))

(event Collision|EventActorBeginOverlap
  (params (OtherActor :type Actor%20Object%20Reference)))

(event EventTick
  (params (DeltaSeconds :type Float%20%28single-precision%29)))

(fn ConstructionScript
  (bind (_zoom _x_offset _y_offset _roll _pitch _yaw _aspect_ratio _field_of_view) (Utilities|Utility-GetCameraSettings))
  (Utilities|Utility-SetCameraSettings (Variables|Default|GetCamera) (Variables|Default|GetSpringArm) (Variables|Controls|GetActor%20to%20Focus) _zoom _x_offset _y_offset _roll _pitch _yaw _aspect_ratio _field_of_view false true))