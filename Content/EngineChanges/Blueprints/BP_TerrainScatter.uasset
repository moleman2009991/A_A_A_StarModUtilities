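; Terrain scatter Blueprint that procedurally places random instances of a set of static meshes around the actor, for debris-style dressing.
; The construction script creates one instanced mesh component per mesh, then uses a seeded stream to scatter instances in an axis-scaled shell with random scale and optional rotation.
; It then configures collision (custom depth stencil when enabled), cull distances and optional forced LOD.
; The UseHISM branch is disconnected.
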(fn ConstructionScript
  (bind _ism_components (Variables|Default|GetISM%20Components))
  (bind _instancedstaticmesh (Variables|Default|GetInstancedStaticMesh))
  (Utilities|FlowControl|Sequence
    (:then_0
      (for _array_element (Variables|Default|GetStatic%20Mesh)
        (bind _returnvalue (AddComponent|AddInstancedStaticMeshComponent false))
        (Utilities|Array|Add (Variables|Default|GetISM%20Components) _returnvalue)
        (Components|StaticMesh|SetStaticMesh _returnvalue _array_element))
      (Variables|Default|SetRandomStream (Math|Random|MakeRandomStream (Variables|Default|GetRandom%20Seed)))
      (for _index (range 0 (Variables|Default|GetInstance%20Count))
        (Components|InstancedStaticMesh|AddInstance (.OutItem (Utilities|Array|RandomFromStream (Variables|Default|GetISM%20Components) (Variables|Default|GetRandomStream))) (Math|Transform|MakeTransform (* (Variables|Default|GetDistance%20Scale%20XYZ) (* (Math|Random|RandomUnitVectorfromStream (Variables|Default|GetRandomStream)) (Math|Random|RandomFloatinRangefromStream (Variables|Default|GetDistance%20Min) (Variables|Default|GetDistance%20Max) (Variables|Default|GetRandomStream)))) (Math|Rotator|SelectRotator (Math|Rotator|MakeRotator 0.0 0.0 (.Yaw (Math|Rotator|BreakRotator (Class|KismetMathLibrary|RandomRotatorfromStream false (Variables|Default|GetRandomStream))))) "0, 0, 0" (Variables|Default|GetEnable%20Random%20Rotation)) (Math|Conversions|ToVector(Float) (* (Math|Random|RandomFloatinRangefromStream (Variables|Default|GetScale%20Min) (Variables|Default|GetScale%20Max) (Variables|Default|GetRandomStream)) (Variables|Default|GetScale%20Uniform)))))))
    (:then_1
      (if (Variables|Default|GetDisable%20Collision%20On%20Debris)
        (for _array_element_2 _ism_components
          (Collision|SetCollisionEnabled _array_element_2 "NoCollision"))
        (else
          (for _array_element_3 _ism_components
            (Collision|SetCollisionEnabled _array_element_3 "QueryAndPhysics")
            ;[1 1 1 1 12] TODO-Damien: Don't think this should be there? But if not, collision doesn't seem to be always properly reneabled...
            (Collision|SetCollisionProfileName _array_element_3 "SimBlockAllStatic" true :!class /Script/Engine.PrimitiveComponent)
            (Utilities|FlowControl|Sequence
              (:then_0
                (Rendering|SetRenderCustomDepth _instancedstaticmesh true))
              (:then_1
                (Rendering|SetCustomDepthStencilValue _instancedstaticmesh 1))
              (:then_2
                (Class|PrimitiveComponent|SetCustomDepthStencilWriteMask _instancedstaticmesh "ERSM_1")))))))
    (:then_2
      (CallFunction|SetMaxDrawDistance))
    (:then_3
      (if (Variables|Default|GetEnable%20Force%20LOD)
        (for _array_element_4 (Variables|Default|GetISM%20Components)
          (Rendering|LOD|SetForcedLodModel _array_element_4 (Variables|Default|GetForced%20LOD)))))))

(fn SetMaxDrawDistance
  (CallFunction|SetMaxDrawDistance (Variables|Rendering|GetCull%20Distances%20Enable) (Variables|Default|GetISM%20Components) (Variables|Rendering|GetCull%20Distances) (Variables|Default|GetScale%20Min) (Variables|Default|GetScale%20Max) (Variables|Default|GetScale%20Uniform) false))