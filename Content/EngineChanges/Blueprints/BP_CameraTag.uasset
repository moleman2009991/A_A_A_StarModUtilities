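; BP_CameraTag is a Blueprint that puts its Tag on the ship that owns it, apparently as a camera-related marker.
; The AddTagtoShip event adds the tag uniquely to the owner's Tags array, and Destroyed removes it again.
; It does no per-frame work, as its Tiir tick getters report ticking disabled with a zero interval.
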(event Custom|Add%20Tag%20to%20Ship
  (Utilities|AddTagstoOwningShip (Variables|Settings|GetTag)))

(event EventDestroyed
  (Utilities|RemoveTagsfromOwningShip (Variables|Settings|GetTag)))

(fn ConstructionScript)

(fn GetTiirTickEnabled
  (return false))

(fn GetTiirTickInterval
  (return 0.0))