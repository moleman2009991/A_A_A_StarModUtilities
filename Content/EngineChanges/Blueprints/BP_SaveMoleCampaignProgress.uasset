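; Campaign progress save object for the Mole campaign, holding the difficulty choice and the persistent fleet option.
; Stores a selected preset (Story, Easy, Medium, Hard or Custom) and resolves it to the matching difficulty settings.
; Each preset has its own variable rather than an array slot, so built-in presets stay read-only while only the Custom settings can be overwritten.
; Simple getters and setters expose the preset and fleet flag.
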(fn SetCustomizedDifficultySettings
  (params (CustomizedCampaignDifficulty :type Campaign%20Difficulty%20Configuration%20Structure))
  (Variables|Default|SetCampaignDifficulty_Custom CustomizedCampaignDifficulty))

(fn GetDifficultySettingsforSelectedPreset
  (bind _difficultysettings (CallFunction|GetDifficultySettingsforPreset (Variables|Default|GetSelectedDifficultyPreset)))
  (return _difficultysettings))

(fn SetDifficultyPreset
  (params (SelectedDifficultyPreset :type ECampaignDifficulty%20Enum :default "Story"))
  (Variables|Default|SetSelectedDifficultyPreset SelectedDifficultyPreset))

(fn GetDifficultySettingsforPreset
  (params (SelectedDifficultyPreset :type ECampaignDifficulty%20Enum :default "Story"))
  (switch Utilities|FlowControl|Switch|SwitchonECampaignDifficulty SelectedDifficultyPreset
    (:Story
      ;[1 1 1] This is done this way so the presets can remain read-only, and the custom setting can be changed, instead of having them all in a single array
      (return (Variables|DifficultyPreset|GetCampaignDifficulty_StoryPreset)))
    (:Easy
      (return (Variables|DifficultyPreset|GetCampaignDifficulty_EasyPreset)))
    (:Medium
      (return (Variables|DifficultyPreset|GetCampaignDifficulty_MediumPreset)))
    (:Hard
      (return (Variables|DifficultyPreset|GetCampaignDifficulty_HardPreset)))
    (:Custom
      (return (Variables|Default|GetCampaignDifficulty_Custom)))))

(fn GetDifficultyPreset
  (return (Variables|Default|GetSelectedDifficultyPreset)))

(fn SetUsePersistentFleet
  (params (UsePersistentFleet :type Boolean))
  (Variables|Default|SetbUsePersistenFleet UsePersistentFleet))

(fn GetUsePersistentFleet
  (return (Variables|Default|GetbUsePersistenFleet)))