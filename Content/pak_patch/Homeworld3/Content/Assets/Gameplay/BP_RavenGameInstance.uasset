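; Raven's game instance, which runs app-wide startup and holds settings, campaign progress and other cross-level state.
; PostInit binds online-service events and preloads ship and weapon data, then initializes UGC, factions, saves, entitlements and progression.
; Network, Shift and platform failures show error dialogs or exit to the main menu, leaving lobbies and logging out as needed.
; PS5-only branches handle temporary saves, session errors and realtime-multiplayer notifications; activity intents route to campaign or multiplayer.
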(event Custom|CE_OnRavenNetworkDisconnected
  (bind _returnvalue (Game|GetGameMode))
  ;[0.003677 0.1221 0.2016] [VTS][WenCongwei][PS5] called when network is disconnected
  ;[1 1 1] [PS5-TRC]R5034 Show dialog after disconnect network
  (Utilities|Casting|CastToBP_LobbyRavenGameMode _returnvalue
    (:then
      _)
    (:CastFailed
      (Utilities|Casting|CastToBP_MultiplayerRavenGameMode _returnvalue
        (:then
          _)
        (:CastFailed
          (Utilities|Casting|CastToBP_MainMenuGameMode _returnvalue)
          (switch Utilities|FlowControl|Switch|SwitchonERavenLoginStatus (Class|RavenOnlineServices|GetLoginStatus (Subsystems|GetRavenOnlineServices))
            (:LoggingIn
              _)
            (:LoggedIn
              _)
            (:Connected
              _)
            (:Authenticated
              _)
            (:NeedReconnect
              _)
            (:Reconnecting
              _))))))
  (Default|DisplayNetworkError :self (CallFunction|GetNetworkErrorWidget) :Message "NetworkError")
  (CallFunction|ExittoMainMenuandLeaveLobby true))

(event Custom|CE_BindOnRavenNetworkDisconnected
  ;[0.003677 0.1221 0.2016] [VTS][WenCongwei][PS5] called when network is disconnected
  (EventDispatchers|AssignOnRavenNetworkDisconnected (Subsystems|GetRavenOnlineServices) (delegate Custom|CE_OnRavenNetworkDisconnected)))

(event Custom|CE_OnRealtimeMultiplayEnd
  (|PS5|RealtimeMultiplayEnd))

(event EventHandleNetworkError
  (params (FailureType :type ENetworkFailure%20Enum :default "NetDriverAlreadyExists") (bIsServer :type Boolean))
  (bind _returnvalue (Game|GetGameMode))
  ;[1 1 1] [PS5-TRC]R5034 Show dialog after disconnect network
  (switch Utilities|FlowControl|Switch|SwitchonENetworkFailure FailureType
    (:ConnectionLost
      (Utilities|Casting|CastToBP_LobbyRavenGameMode _returnvalue
        (:then
          _)
        (:CastFailed
          (Utilities|Casting|CastToBP_MultiplayerRavenGameMode _returnvalue
            (:then
              _)
            (:CastFailed
              (Utilities|Casting|CastToBP_MainMenuGameMode _returnvalue)
              (switch Utilities|FlowControl|Switch|SwitchonERavenLoginStatus (Class|RavenOnlineServices|GetLoginStatus (Subsystems|GetRavenOnlineServices))
                (:LoggingIn
                  _)
                (:LoggedIn
                  _)
                (:Connected
                  _)
                (:Authenticated
                  _)
                (:NeedReconnect
                  _)
                (:Reconnecting
                  _))))))
      (Default|DisplayNetworkError :self (CallFunction|GetNetworkErrorWidget) :Message "NetworkError")
      (CallFunction|ExittoMainMenuandLeaveLobby true))))

(event EventInit)

(event EventPostInit
  (Utilities|FlowControl|Sequence
    (:then_0
      (|InitTempSaveGameOnPS5))
    (:then_1
      (|BindEventOnPS5))
    (:then_2
      (|BindShiftEvent))
    (:then_3
      (|BindOnExitToMainMenu))
    (:then_4
      (|DoInitialization))))

(event EventShutdown
  (Class|AkGameplayStatics|PostEventatLocation "/Game/WwiseAudio/Events/Game_Flow/Game_Flow/stop_all.stop_all" "0, 0, 0" "0, 0, 0"))

(fn SetGameSettings
  (params (GameSettings :type BP%20Save%20Game%20Settings%20Object%20Reference))
  (bind _output_get (Variables|Default|SetGameSettings GameSettings))
  (Class|RavenGameInstance|PropagateGameSettingstoCPP _output_get))

(fn LoadGameSettings
  (params (EmitEvents :type Boolean))
  (bind _returnvalue (SaveGame|LoadGamefromSlot (Variables|Default|GetGameSettingsSlotName)))
  (bind _asbp_save_game_settings (Utilities|Casting|CastToBP_SaveGameSettings _returnvalue)
    (:then
      ;[1 1 1] Fix up old settings file based on version written in "SaveGameSettings"
      (bind _save_output (CallFunction|ProcessLoadedSettings _asbp_save_game_settings))
      (if (Utilities|IsValid _save_output)
        (CallFunction|SetGameSettings _asbp_save_game_settings) ; Must refresh var, as this will\nhave previously-saved settings
        (if EmitEvents
          (Default|CallGameSettingsLoaded _asbp_save_game_settings) ; DOES NOT FIRE IF GAME IS PAUSED!
          (Class|RavenGameInstance|BroadcastSettingsLoadedNative)
          (CallFunction|BroadcastNLIPSSettingsChange))
        (else
          (bind _returnvalue_2 (SaveGame|CreateSaveGameObject "/Game/GameModes/MainMenu/Blueprints/BP_SaveGameSettings.BP_SaveGameSettings_C" :!label _label))
          (CallFunction|SetGameSettings _returnvalue_2)
          (CallFunction|SaveGameSettings false))))
    (:CastFailed
      (goto _label))))

(fn SaveGameSettings
  (params (EmitEvents :type Boolean))
  (bind _gamesettings (Variables|Default|GetGameSettings))
  ;[1 1 1] This is where we write the current settings file version
  (Variables|/Game/GameModes/MainMenu/Blueprints/BP_SaveGameSettings.BP_SaveGameSettings_C|SetSaveVersion _gamesettings 1)
  (bind _returnvalue (SaveGame|SaveGametoSlot _gamesettings (Variables|Default|GetGameSettingsSlotName))) ; The function containing this logic is called\nexternally when values need to be saved:\nthe game instance doesn't normally save\non its own
  (if _returnvalue
    (if EmitEvents
      (Default|CallGameSettingsSaved _gamesettings) ; DOES NOT FIRE IF GAME IS PAUSED!
      (Class|RavenGameInstance|BroadcastSettingsSavedNative))
    (CallFunction|SendCameraSettingsTelemetry (CallFunction|GetRavenGameInstancePure))
    (CallFunction|BroadcastNLIPSSettingsChange)
    (else
      (Development|PrintString "Failed to save game settings!"))))

(fn LoadCampaignProgress
  (params (EmitEvents :type Boolean))
  (bind _returnvalue (Class|RTSSaveGameSubsystem|LoadProfileSave (Subsystems|GetRTSSaveGameSubsystem)))
  (bind _asbp_save_campaign_progress (Utilities|Casting|CastToBP_SaveCampaignProgress (Variables|/Script/Raven.ProfileSaveGame|GetCampaignProgress _returnvalue))
    (:then
      (bind _output_get (Variables|Default|SetCampaignProgress _asbp_save_campaign_progress)) ; Must refresh var, as this will\nhave previously-saved settings
      (if EmitEvents
        (Default|CallCampaignProgressLoaded _output_get)))
    (:CastFailed
      (Development|PrintString "Faled to load campaign progress!"))))

(fn SaveCampaignProgress
  (params (MasterLevelName :type String) (EmitEvents :type Boolean))
  (bind _campaignprogress (Variables|Default|GetCampaignProgress))
  (if (Utilities|Array|IsEmpty MasterLevelName) ; Save without adjusting anything\nhere if no mission specified
    (Class|RTSSaveGameSubsystem|StoreProfileSave (Subsystems|GetRTSSaveGameSubsystem) :!label _label)
    (if EmitEvents
      (Default|CallCampaignProgressSaved _campaignprogress))
    (else
      ;[1 1 1] Find Mission Index
      (bind _outrownames (DataTable|GetDataTableRowNames (Variables|Default|GetCampaignLevelData))) ; Dump campaign row names to array
      (if (== (Utilities|Array|FindItem _outrownames (Utilities|String|StringToName MasterLevelName)) -1)
        (Development|PrintString "Couldn't find mission!")
        (else
          ;[1 1 1] Update HardestDifficultyCompleted
          (bind _asrtsgame_state (Utilities|Casting|CastToRTSGameState (Game|GetGameState))
            (:then
              (bind _asbp_raven_scenario_parameters (Utilities|Casting|CastToBP_Raven_ScenarioParameters (Variables|/Script/Raven.RTSGameState|GetParameters _asrtsgame_state))
                (:then
                  (Class|SaveCampaignProgress|UpdateDifficultyCompleted _campaignprogress MasterLevelName (Default|GetDifficultyPreset _asbp_raven_scenario_parameters)))
                (:CastFailed
                  (Development|PrintString "Couldn't find current mission difficulty." :!label _label_2))))
            (:CastFailed
              (goto _label_2)))
          ;[1 1 1] Update LastCompletedMissionIndex
          (Variables|/Script/Raven.SaveCampaignProgress|SetMostRecentCompletedMissionIndex _campaignprogress (+ (Utilities|Array|FindItem _outrownames (Utilities|String|StringToName MasterLevelName)) 1))
          (if (> (+ (Utilities|Array|FindItem _outrownames (Utilities|String|StringToName MasterLevelName)) 1) (Variables|/Game/GameModes/MainMenu/Blueprints/BP_SaveCampaignProgress.BP_SaveCampaignProgress_C|GetLastCompletedMissionIndex _campaignprogress)) ; If new index is larger than current, set it and save it
            (bind _output_get (Variables|/Game/GameModes/MainMenu/Blueprints/BP_SaveCampaignProgress.BP_SaveCampaignProgress_C|SetLastCompletedMissionIndex _campaignprogress (+ (Utilities|Array|FindItem _outrownames (Utilities|String|StringToName MasterLevelName)) 1)))
            (Development|PrintString (Utilities|String|ToString(Text) (Utilities|Text|FormatText "Campaign progress set to level index: {LevelIndex}" _output_get)))
            (goto _label)
            (else
              (Development|PrintString "Campaign progress not updated"))))))))

(fn ResetCampaignProgress
  (bind _campaignprogress (Variables|Default|GetCampaignProgress))
  (Variables|/Game/GameModes/MainMenu/Blueprints/BP_SaveCampaignProgress.BP_SaveCampaignProgress_C|SetLastCompletedMissionIndex _campaignprogress 0) ; Set to 0
  (Utilities|Map|Clear (Variables|/Script/Raven.SaveCampaignProgress|GetHardestDifficultyCompleted _campaignprogress))
  (Class|RTSSaveGameSubsystem|StoreProfileSave (Subsystems|GetRTSSaveGameSubsystem)))

(fn InitUGC
  (bind _returnvalue (Game|ConstructObjectfromClass "/Script/SimpleUGC.UGCRegistry" self))
  (bind _output_get (Variables|UGC|SetUGCRegistry _returnvalue))
  (bind _returnvalue_2 (Class|UGCRegistry|FindUGCPackages _output_get))
  (if _returnvalue_2
    (Development|PrintText (Utilities|Text|FormatText "UGC: found {num_packages} packages." (Utilities|Array|Length (Variables|/Script/SimpleUGC.UGCRegistry|GetUGCPackages _output_get))) false)))

(fn PreloadSoftObjectReferences
  (bind _returnvalue (Development|GetConsoleVariableIntValue "sim.ProxyPreloadType"))
  (switch Utilities|FlowControl|Switch|SwitchonESimPreloadType (Utilities|Enum|ByteToEnumESimPreloadType (Math|Conversions|ToByte(Integer) _returnvalue))
    (:NoPreload
      (return))
    (:SyncPreloadInGameInstance
      _)
    (:AsyncPreloadInGameInstance
      _))
  (bind _loadedassets (Class|EntityStaticDataAssetFunctionLibrary|PreloadSoftObjectReferences "/Script/RavenSimulation.ShipStaticData"))
  (Variables|Default|SetPreloadedShips _loadedassets)
  (bind _loadedassets_2 (Class|EntityStaticDataAssetFunctionLibrary|PreloadSoftObjectReferences "/Script/RavenSimulation.WeaponFireStaticData"))
  (Variables|Default|SetPreloadedWeapons _loadedassets_2))

(fn IsinGame
  (Utilities|Casting|CastToRavenGameMode (Game|GetGameMode) ; I don't believe we use any other game mode during gameplay\nbut if we do, we'll need to modify this to:\nif (RavenGameMode or OtherGameMode)
    (:then
      (return true))
    (:CastFailed
      (return false))))

(fn ApplyGameUserSettings
  (bind _returnvalue (Settings|GetGameUserSettings))
  (bind _asbp_raven_game_user_settings (Utilities|Casting|CastToBP_RavenGameUserSettings _returnvalue))
  (Default|ApplyConfigVariableSettings _asbp_raven_game_user_settings (CallFunction|IsinGame)))

(fn OnActivityIntentReceivedDelegate
  (params (ActivtyType :type EActivityType%20Enum :default "Campaign"))
  (bind _returnvalue (Game|GetPlayerController 0))
  (bind _returnvalue_2 (HUD|GetHUD _returnvalue))
  ;[1 1 1] VTS|PS5|When entering the activity, exit the previous session
  (switch Utilities|FlowControl|Switch|SwitchonEActivityType ActivtyType
    (:Campaign
      (Class|RavenOnlineServices|LeaveLobbySession (Subsystems|GetRavenOnlineServices) (Game|GetPlayerController 0))
      (|PremiumFeature|RealtimeEnd)
      ;[1 1 1] [PS5][WangKejin] Load the most recent save data
      (bind (_saveid _levelname _returnvalue_3) (Class|RTSSaveGameSubsystem|PS5FindMostRecentSaveData (Subsystems|GetRTSSaveGameSubsystem)))
      (if _returnvalue_3 ; Check if  campaign save file exists
        ;;[1 1 1] Load Save Game
        (Class|RTSSaveGameSubsystem|SetSaveGametoLoadforNextLevel (Subsystems|GetRTSSaveGameSubsystem) _saveid)
        (Class|RavenOnlineChunkInstallSubsystem|OpenLevelwithCheck (Subsystems|GetRavenOnlineChunkInstallSubsystem) _levelname)
        (else
          (Class|GameplayStatics|CancelAsyncLoading)
          (Game|OpenLevel(byName) "Tutorial_Main"))))
    (:Multiplayer
      (Utilities|Casting|CastToBP_MainMenuHUD _returnvalue_2
        (:then
          (Default|CallOnMultiplayerActivity))
        (:CastFailed
          (Variables|Default|SetIsPrepared true)
          (bind _asbp_lobby_raven_hud (Utilities|Casting|CastToBP_LobbyRavenHUD _returnvalue_2)
            (:then
              (Default|ActivityLeaveLobby _asbp_lobby_raven_hud))
            (:CastFailed
              (Class|GameplayStatics|CancelAsyncLoading)
              (Game|OpenLevel(byName) "MainMenu")
              (|PS5|RealtimeMutliplay_2))))))))

(fn ShowErrorandExittoMainMenu
  (params (ErrorLog :type String) (DialogMsg :type Text))
  (Development|PrintString ErrorLog true true "(R=0.894422,G=0.000000,B=1.000000,A=1.000000)" 6.0)
  (Default|DisplayNetworkError :self (CallFunction|GetNetworkErrorWidget) :Message DialogMsg)
  (CallFunction|ExittoMainMenu))

(fn ResetChallengeProgress
  (params (Row%20Name :type Data%20Table%20Row%20Handle%20Structure)))

(fn IsMultiplayerRunActive
  (return (Variables|Multiplayer|GetbIsMultiplayerRunActive)))

(fn ShowExittoMainMenuReasonifExists
  (CallFunction|ShowExittoMainMenuErrorMessage (Variables|Multiplayer|GetExitToMainMenuReason))
  (Variables|Multiplayer|SetExitToMainMenuReason "NoReason"))

(fn ShowLobbyTaskErrorifExists
  (CallFunction|ShowLobbyTaskErrorMessage (Variables|Multiplayer|GetExitToMainMenuLobbyTaskError))
  (Variables|Multiplayer|SetExitToMainMenuLobbyTaskError "NoError"))

(fn ExittoMainMenufromLobbyTaskError
  (params (LobbyError :type ELobbyTaskError%20Enum :default "NoError") (Need%20to%20Logout :type Boolean))
  (Variables|Multiplayer|SetExitToMainMenuLobbyTaskError LobbyError)
  (CallFunction|ExittoMainMenuandLeaveLobby Need%20to%20Logout))

(fn ReceiveLevelNametoLevelTitle
  (params (levelName :type String))
  (bind _returnvalue (Utilities|Text|MakeLiteralText "Unknown Mission"))
  (bind _returnvalue_2 (Utilities|GetDataTableRow "/Game/GameModes/MainMenu/Blueprints/DT_CampaignLevelData.DT_CampaignLevelData" (Utilities|String|StringToName levelName))
    (:then
      (return (.title _returnvalue_2)))
    (:RowNotFound
      (Class|RavenMessageLogUtilsFunctionLibrary|RavenMessageLogError (Utilities|String|ToString(Text) (Utilities|Text|FormatText "Level Name {0} missing from DT_CampaignLevelData. Returning \"{1}\" instead." levelName _returnvalue)) (Utilities|GetClassDisplayName (Utilities|GetClass self)))
      (return _returnvalue))))

(fn ApplyGamma
  (Development|ExecuteConsoleCommand (Utilities|String|Append "gamma " (Utilities|String|ToString(Float) (Variables|/Script/Raven.RavenGameUserSettings|GetGamma (CallFunction|GetRavenGameUserSettings)))) 0))

(fn SetLatestTeamID
  (params (NewTeamID :type Integer))
  (Variables|Multiplayer|SetLatestTeamID NewTeamID))

(fn SaveBenchmarkingData
  (params (FPSData :type Benchmarking%20Data%20Structure) (CPUData :type Benchmarking%20Data%20Structure) (GFXData :type Benchmarking%20Data%20Structure) (MemoryUsage :type Benchmarking%20Data%20Structure))
  (bind _benchmarkingdata (Variables|Default|GetBenchmarkingData))
  (Utilities|Array|Clear _benchmarkingdata)
  (Utilities|Array|SetArrayElem _benchmarkingdata 0 FPSData true)
  (Utilities|Array|SetArrayElem _benchmarkingdata 1 CPUData true)
  (Utilities|Array|SetArrayElem _benchmarkingdata 2 GFXData true)
  (Utilities|Array|SetArrayElem _benchmarkingdata 3 MemoryUsage true))

(fn LoadBenchmarkingData
  (bind _benchmarkingdata (Variables|Default|GetBenchmarkingData))
  (return (Utilities|Array|Get(acopy) _benchmarkingdata) (Utilities|Array|Get(acopy) _benchmarkingdata 1) (Utilities|Array|Get(acopy) _benchmarkingdata 2) (Utilities|Array|Get(acopy) _benchmarkingdata 3)))

(fn ReinitGameSettings
  (params (OnlyReinitializeExistingWidgets :type Boolean))
  (Default|CallGameSettingsReinitialized OnlyReinitializeExistingWidgets))

(fn ProcessLoadedSettings
  (params (Save%20Input :type BP%20Save%20Game%20Settings%20Object%20Reference))
  (if (== 0 (Variables|/Game/GameModes/MainMenu/Blueprints/BP_SaveGameSettings.BP_SaveGameSettings_C|GetSaveVersion Save%20Input)) ; Intentionally discard saved settings at version 0, RAVEN-18516
    (return 0)
    (else
      (return Save%20Input))))

(fn BroadcastNLIPSSettingsChange
  (bind _gamesettings (Variables|Default|GetGameSettings))
  (bind _asraven_player_controller (Utilities|Casting|CastToRavenPlayerController (Game|GetPlayerController 0)))
  (Default|CallOnNLIPSSettingsChanged (Variables|/Game/Assets/Gameplay/RavenPlayerController.RavenPlayerController_C|GetEventDispatcherComponent _asraven_player_controller) (Variables|/Game/GameModes/MainMenu/Blueprints/BP_SaveGameSettings.BP_SaveGameSettings_C|GetIsNLIPSEnabled _gamesettings) (Variables|/Game/GameModes/MainMenu/Blueprints/BP_SaveGameSettings.BP_SaveGameSettings_C|GetNLIPSScale _gamesettings)))

(event Custom|CE_OnPlatformSessionError
  (params (ErrorMessage :type Text))
  ;[0.003677 0.1221 0.2016] [VTS][WenCongwei][PS5] called when a platform session error occurs
  (Default|DisplayNetworkError :self (CallFunction|GetNetworkErrorWidget) :Message ErrorMessage))

(event Custom|CE_OnRavenPlatformLogin
  (params (LocalUserNum :type Integer) (UniquePlayerId :type String))
  ;[0.003922 0.1216 0.2] [VTS][WenCongwei][PS5][RAVEN-2482] called on login status changed
  (Development|PrintString (Utilities|String|BuildString(Integer) UniquePlayerId "(UniquePlayerId) " LocalUserNum "(Local User Num) Login ") true true "(R=0.894422,G=0.000000,B=1.000000,A=1.000000)" 6.0))

(event Custom|CE_OnRavenPlatformLogout
  ;[0.003922 0.1216 0.2] [VTS][WenCongwei][PS5][RAVEN-2482] called on login status changed
  (Development|PrintString "[RavenOnlineServices] OnRavenLogout" true true "(R=0.894422,G=0.000000,B=1.000000,A=1.000000)" 6.0)
  (Default|DisplayNetworkError :self (CallFunction|GetNetworkErrorWidget) :Message "NetworkError_PlatformLogout")
  (CallFunction|ExittoMainMenuandLeaveLobby true))

(event Custom|CE_OnShiftConnectionLost
  (bind _returnvalue (Game|GetGameMode))
  (Variables|Multiplayer|SetIsNeedShiftReconnect true)
  (Class|RavenOnlineServices|Logout (Subsystems|GetRavenOnlineServices) (Game|GetPlayerController 0))
  (if (or (.bSuccess (Utilities|Casting|CastToBP_MultiplayerRavenGameMode _returnvalue)) (.bSuccess (Utilities|Casting|CastToBP_LobbyRavenGameMode _returnvalue)))
    (CallFunction|ShowErrorandExittoMainMenu "[RavenOnlineServices] OnShiftConnectionLost" "ShiftConnectionLostMessage")))

(event Custom|CE_OnShiftSessionAutoLogout
  (CallFunction|ShowErrorandExittoMainMenu "[RavenOnlineServices] OnShiftSessionAutoLogout" "ShiftLogoutMessage"))

(event Custom|CE_OnExitToMainMenu
  (params (IsNeedToLogout :type Boolean) (ExitToMainMenuReason :type EExitToMainMenuReason%20Enum :default "ShiftPresenceUnavailable"))
  ;[0 0.1216 0.2] [VTS][WenCongwei] on exit to main menu
  (Development|PrintString (Utilities|String|Append "[RavenOnlineServices] OnExitToMainMenu Reason: " (Utilities|String|EnumtoString ExitToMainMenuReason)) true true "(R=0.894422,G=0.000000,B=1.000000,A=1.000000)" 6.0)
  (Variables|Multiplayer|SetExitToMainMenuReason ExitToMainMenuReason)
  (CallFunction|ExittoMainMenuandLeaveLobby IsNeedToLogout))

(event Custom|ExitToMainMenuAndLeaveLobby
  (params (NeedToLogout :type Boolean))
  (bind _returnvalue (Game|GetGameMode))
  (bind _returnvalue_2 (Game|GetPlayerController 0))
  (bind _returnvalue_3 (Game|GetGameMode))
  (bind _returnvalue_4 (Game|GetPlayerController 0))
  (bind _returnvalue_5 (Subsystems|GetRavenOnlineServices))
  (Class|PlatformInfoSubsystem|CheckIsPlatformasExec (|PlatformInfoSubsystem) "PS5"
    (:True
      (Utilities|FlowControl|Sequence
        (:then_0
          (CallFunction|CEonRealtimeMultiplayEnd))
        (:then_1
          (Utilities|Casting|CastToBP_MultiplayerRavenGameMode _returnvalue
            (:then
              (|LeaveLocalRavenLobby _returnvalue_5 _returnvalue_4 true :!label _label
                (:then
                  (CallFunction|ExittoMainMenu)
                  (if NeedToLogout
                    (Class|RavenOnlineServices|Logout _returnvalue_5 _returnvalue_4 :!label _label_2)))))
            (:CastFailed
              (Utilities|Casting|CastToBP_LobbyRavenGameMode _returnvalue
                (:then
                  (goto _label))
                (:CastFailed
                  (goto _label_2))))))))
    (:False
      (Utilities|Casting|CastToBP_MultiplayerRavenGameMode _returnvalue_3
        (:then
          (|LeaveLocalRavenLobby _returnvalue_5 _returnvalue_2 true :!label _label_3
            (:OnComplete
              _)))
        (:CastFailed
          (Utilities|Casting|CastToBP_LobbyRavenGameMode _returnvalue_3
            (:then
              (goto _label_3))
            (:CastFailed
              _))))
      (CallFunction|ExittoMainMenu)
      (if NeedToLogout
        (Class|RavenOnlineServices|Logout _returnvalue_5 _returnvalue_2)))))