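; Drone Frigate unit Blueprint that makes a drone pop-cap artifact obtainable from the ship while it is alive.
; On BeginPlay it attaches the artifact and watches its own entity through a group death task, which removes the artifact and shuts down on death.
; ShouldRedirectCommandBP redirects commands to the Parent selectable whenever that parent can accept them.
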(event EventBeginPlay
  (bind _self self)
  (bind _group (Variables|Default|GetGroup))
  (bind _returnvalue (Class|TiirEntityFunctionLibrary|GetEntity _self))
  (|CallParentFunction)
  (Class|TiirEntityFunctionLibrary|AddObtainableArtifacttoShip _returnvalue "/Game/Assets/Tunables/Artifacts/Base/Artifact_PopCap_Drones.Artifact_PopCap_Drones")
  (Class|TiirEntityGroupFunctionLibrary|GroupAddEntity _group _returnvalue)
  (bind _task (|TaskWaitforDeath _group)
    (:OnDeath
      (Class|TiirEntityFunctionLibrary|RemoveObtainableArtifactfromShip _returnvalue)
      (Class|TiirAsyncTaskBase|TaskShutdown _task))))

(event Collision|EventActorBeginOverlap
  (params (OtherActor :type Actor%20Object%20Reference)))

(event EventTick
  (params (DeltaSeconds :type Float%20%28single-precision%29))
  (|CallParentFunction DeltaSeconds) ; This node is disabled and will not be called.\nDrag off pins to build functionality.
)

(fn ConstructionScript
  (|CallParentFunction))

(fn ShouldRedirectCommandBP
  (params (InOutTargets :type Array%20of%20Raven%20Selectable%20Interfaces) (CommandSettings :type Object%20Object%20Reference))
  (bind _parent (Variables|Default|GetParent))
  (bind _asraven_selectable (Utilities|Casting|CastToRavenSelectable _parent))
  (if (Class|RavenSelectable|CanAcceptCommand _asraven_selectable CommandSettings)
    (Utilities|Array|Add InOutTargets _asraven_selectable)
    (return true)
    (else
      (return false))))